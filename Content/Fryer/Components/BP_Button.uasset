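; BP_Button is a clickable, labeled button actor among the Fryer components that plays an animation when pressed.
; Construction copies its Text variable to the TextRenderer, and BeginPlay enables player input.
; Clicks and the Excute and Demonstrate events all run the ClickAnimation sequence through Play.
; When the sequence player finishes, the button fires OnCompleted to signal that the action is done.
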(event Custom|OnFinished_Event
  (Default|CallOnCompleted))

(event EventBeginPlay
  (Input|EnableInput (Game|GetPlayerController 0))
  (EventDispatchers|AssignOnFinished (Variables|/Script/ActorSequence.ActorSequenceComponent|GetSequencePlayer (Variables|Default|GetClick%20Animation)) (delegate Custom|OnFinished_Event)))

(event EventExcute
  (CallFunction|Play))

(event EventTick
  (params (DeltaSeconds :type Float%20%28single-precision%29)))

(event MouseInput|EventActorOnClicked
  (params (ButtonPressed :type Key%20Structure :default "None"))
  (CallFunction|Play))

(event EventDemonstrate
  (CallFunction|Play))

(fn ConstructionScript
  (Rendering|Components|TextRender|SetText (Variables|Default|GetTextRenderer) (Variables|Default|GetText)))

(fn Play
  (Class|ActorSequenceComponent|PlaySequence (Variables|Default|GetClick%20Animation)))