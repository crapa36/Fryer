(event Custom|OnFinished_Event
  (Variables|Default|SetAnim%20Done? true))

(event Custom|On%20Wash%20Button%20Clicked
  (Variables|Default|SetIdx (- (Utilities|Array|Length (Variables|Default|GetStates)) 1))
  (if (Variables|Default|GetAnim%20Done?)
    (CallFunction|Play)
    (Variables|Default|SetIdx 0)
    (Variables|Default|SetReady? false)))

(event EventBeginPlay
  (Input|EnableInput (Game|GetPlayerController 0))
  (for _array_element (Actor|GetComponentsByClass "/Script/ActorSequence.ActorSequenceComponent")
    (EventDispatchers|AssignOnFinished (Variables|/Script/ActorSequence.ActorSequenceComponent|GetSequencePlayer _array_element) (delegate Custom|OnFinished_Event))))

(event MouseInput|EventActorOnClicked
  (params (ButtonPressed :type Key%20Structure :default "None"))
  (if (and (Variables|Default|GetAnim%20Done?) (not (Variables|Default|GetReady?)))
    (Utilities|FlowControl|Sequence
      (:then_0
        (CallFunction|Play))
      (:then_1
        (CallFunction|NextAnim)))))

(event EventTick
  (params (DeltaSeconds :type Float%20%28single-precision%29)))

(fn ConstructionScript)

(fn Play
  (Variables|Default|SetAnim%20Done? false)
  (switch string (Utilities|Array|Get(acopy) (Variables|Default|GetStates) (Variables|Default|GetIdx))
    (:Out
      (Class|ActorSequenceComponent|PlaySequence (Variables|Default|GetOut%20Box)))
    (:In
      (Class|ActorSequenceComponent|PlaySequence (Variables|Default|GetIn%20Box)))
    (:Fill
      (Class|ActorSequenceComponent|PlaySequence (Variables|Default|GetFill%20Water)))
    (:Drain
      (Class|ActorSequenceComponent|PlaySequence (Variables|Default|GetDrain%20Water)))
    (:Open
      (Class|ActorSequenceComponent|PlaySequence (Variables|Default|GetOpen%20Cap)))
    (:Close
      (Class|ActorSequenceComponent|PlaySequence (Variables|Default|GetClose%20Cap)))))

(fn NextAnim
  (if (not (Variables|Default|GetReady?))
    (bind _output_get (Variables|Default|SetIdx (+ (Variables|Default|GetIdx) 1)))
    (if (== _output_get (- (Utilities|Array|Length (Variables|Default|GetStates)) 1))
      (Variables|Default|SetReady? true))))