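; BP_Glowing is a Blueprint that drives a pulsing glow value, toggled by its On and Off events.
; While Glowing is set, Tick moves Amount back and forth linearly between zero and one, flipping the Increase flag and clamping at each end.
; Off freezes Amount at its current value, and the graph itself does not apply the value to any material or light.
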(event EventBeginPlay)

(event EventTick
  (params (DeltaSeconds :type Float%20%28single-precision%29))
  (bind _returnvalue (* DeltaSeconds 1.0))
  (if (Variables|Default|GetGlowing?)
    (if (Variables|Default|GetIncrease?)
      (if (>= (+ (Variables|Default|GetAmount) _returnvalue) 1.0)
        (Variables|Default|SetIncrease? false)
        (Variables|Default|SetAmount (Math|Float|Clamp(Float) (+ (Variables|Default|GetAmount) _returnvalue)))
        (else
          (Variables|Default|SetAmount (+ (Variables|Default|GetAmount) _returnvalue))))
      (elif (<= (- (Variables|Default|GetAmount) _returnvalue) 0.0)
        (Variables|Default|SetIncrease? true)
        (Variables|Default|SetAmount (Math|Float|Clamp(Float) (- (Variables|Default|GetAmount) _returnvalue)))
        (else
          (Variables|Default|SetAmount (- (Variables|Default|GetAmount) _returnvalue)))))))

(event EventOff
  (Variables|Default|SetGlowing? false))

(event EventOn
  (Variables|Default|SetGlowing? true))