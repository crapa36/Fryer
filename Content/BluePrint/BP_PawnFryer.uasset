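; BP_PawnFryer is a fryer pawn with washing and cooking buttons, built from child actors.
; On BeginPlay it caches its clean and dirty water boxes and basket, then binds both buttons' completion events.
; The wash button notifies both water boxes.
; The cook button plays a looping sequence, guarded by AnimDone so it cannot restart until the sequence player reports finished.
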(event Custom|OnCompleted_StartButton_Event
  (CallFunction|PlayCookAnim))

(event Custom|OnFinished_Event
  (Variables|Default|SetAnim%20Done? true))

(event Custom|OnCompleted_CleanButton_Event
  (Default|OnWashButtonClicked (Variables|Default|GetClean%20WaterBox%20Actor)))

(event EventBeginPlay
  (CallFunction|CastChildActor)
  (bind _asbp_button (Utilities|Casting|CastToBP_Button (Variables|/Script/Engine.ChildActorComponent|GetChildActor (Variables|Default|GetWashingButton))))
  (EventDispatchers|AssignOnCompletedCleanButton _asbp_button (delegate Custom|OnCompleted_CleanButton_Event))
  (bind _asbp_button_2 (Utilities|Casting|CastToBP_Button (Variables|/Script/Engine.ChildActorComponent|GetChildActor (Variables|Default|GetCookingButton))))
  (EventDispatchers|AssignOnCompletedStartButton _asbp_button_2 (delegate Custom|OnCompleted_StartButton_Event))
  (EventDispatchers|AssignOnFinished (Variables|/Script/ActorSequence.ActorSequenceComponent|GetSequencePlayer (Variables|Default|GetCooking%20Anim)) (delegate Custom|OnFinished_Event)))

(event Collision|EventActorBeginOverlap
  (params (OtherActor :type Actor%20Object%20Reference)))

(event EventTick
  (params (DeltaSeconds :type Float%20%28single-precision%29)))

(fn ConstructionScript)

(fn CastChildActor
  (bind _asbp_water_box (Utilities|Casting|CastToBP_WaterBox (Variables|/Script/Engine.ChildActorComponent|GetChildActor (Variables|Default|GetCleanWaterBox)))
    (:then
      (Variables|Default|SetClean%20WaterBox%20Actor _asbp_water_box)
      (bind _asbp_water_box_2 (Utilities|Casting|CastToBP_WaterBox (Variables|/Script/Engine.ChildActorComponent|GetChildActor (Variables|Default|GetDirtyWaterBox))))
      (Variables|Default|SetDirty%20WaterBox%20Actor _asbp_water_box_2)
      (bind _asbp_basket (Utilities|Casting|CastToBP_Basket (Variables|/Script/Engine.ChildActorComponent|GetChildActor (Variables|Default|GetBasket))))
      (Variables|Default|SetBasket%20Actor _asbp_basket))
    (:CastFailed
      _))
  (return))

(fn PlayCookAnim
  (if (Variables|Default|GetAnim%20Done?)
    (Variables|Default|SetAnim%20Done? false)
    (Class|MovieSceneSequencePlayer|PlayLooping (Variables|/Script/ActorSequence.ActorSequenceComponent|GetSequencePlayer (Variables|Default|GetCooking%20Anim)) 2)))