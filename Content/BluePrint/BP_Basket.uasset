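; BP_Basket is a clickable basket actor that alternates between an In and an Out animation sequence.
; A click or the Excute event calls Play, which runs one sequence and flips a toggle for the next call.
; An AnimDone flag blocks replays until the sequence finishes.
; Each sequence's finish callback resets that flag and fires the matching basket In or Out completed dispatcher.
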(event Custom|In%20Anim%20OnFinished
  (Default|CallOnCompletedBasketin)
  (Variables|Default|SetAnim%20Done? true))

(event Custom|Out%20Anim%20OnFinished
  (Default|CallOnCompletedBasketOut)
  (Variables|Default|SetAnim%20Done? true))

(event EventBeginPlay
  (Input|EnableInput (Game|GetPlayerController 0))
  (EventDispatchers|AssignOnFinished (Variables|/Script/ActorSequence.ActorSequenceComponent|GetSequencePlayer (Variables|Default|GetIn%20Animation)) (delegate Custom|In%20Anim%20OnFinished))
  (EventDispatchers|AssignOnFinished (Variables|/Script/ActorSequence.ActorSequenceComponent|GetSequencePlayer (Variables|Default|GetOut%20Animation)) (delegate Custom|Out%20Anim%20OnFinished)))

(event EventExcute
  (CallFunction|Play))

(event EventTick
  (params (DeltaSeconds :type Float%20%28single-precision%29)))

(event MouseInput|EventActorOnClicked
  (params (ButtonPressed :type Key%20Structure :default "None"))
  (CallFunction|Play))

(fn ConstructionScript)

(fn Play
  (if (Variables|Default|GetAnim%20Done?)
    (Utilities|FlowControl|Sequence
      (:then_0
        (Variables|Default|SetAnim%20Done? false))
      (:then_1
        (if (Variables|Default|GetAnim%20Toogle)
          (Class|ActorSequenceComponent|PlaySequence (Variables|Default|GetOut%20Animation))
          (else
            (Class|ActorSequenceComponent|PlaySequence (Variables|Default|GetIn%20Animation)))))
      (:then_2
        (Variables|Default|SetAnim%20Toogle (not (Variables|Default|GetAnim%20Toogle)))))))