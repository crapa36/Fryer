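; Fryer basket actor that animates moving in and out through two sequence components, InAnimation and OutAnimation.
; A click or Excute alternates between the two, with AnimDone blocking new plays until the current sequence finishes and fires its basket-in or basket-out completion dispatcher.
; Demonstrate chains out then in through a temporary finish binding, while Reset stops both sequences and restores the transform saved at BeginPlay.
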(event Custom|In%20Anim%20OnFinished
  (Default|CallOnCompletedBasketin)
  (Variables|Default|SetAnim%20Done? true))

(event Custom|Out%20Anim%20OnFinished
  (Default|CallOnCompletedBasketOut)
  (Variables|Default|SetAnim%20Done? true))

(event Custom|OnFinished_Event
  (EventDispatchers|UnbindEventfromOnFinished (Variables|/Script/ActorSequence.ActorSequenceComponent|GetSequencePlayer (Variables|Default|GetOut%20Animation)) (delegate Custom|OnFinished_Event))
  (Class|ActorSequenceComponent|PlaySequence (Variables|Default|GetIn%20Animation)))

(event Custom|OnPlay_Event
  (Variables|Default|SetAnim%20Done? false))

(event Custom|OnPlay_Event_0
  (Variables|Default|SetAnim%20Done? false))

(event EventBeginPlay
  (bind _out_animation (Variables|Default|GetOut%20Animation))
  (bind _in_animation (Variables|Default|GetIn%20Animation))
  (bind _sequenceplayer (Variables|/Script/ActorSequence.ActorSequenceComponent|GetSequencePlayer _in_animation))
  (bind _sequenceplayer_2 (Variables|/Script/ActorSequence.ActorSequenceComponent|GetSequencePlayer _out_animation))
  (Variables|Default|SetStart%20Trans (Transformation|GetActorTransform))
  (Input|EnableInput (Game|GetPlayerController 0))
  (EventDispatchers|AssignOnFinished _sequenceplayer (delegate Custom|In%20Anim%20OnFinished))
  (EventDispatchers|AssignOnPlay _sequenceplayer (delegate Custom|OnPlay_Event))
  (EventDispatchers|AssignOnFinished _sequenceplayer_2 (delegate Custom|Out%20Anim%20OnFinished))
  (EventDispatchers|AssignOnPlay _sequenceplayer_2 (delegate Custom|OnPlay_Event_0)))

(event EventExcute
  (CallFunction|Play))

(event EventTick
  (params (DeltaSeconds :type Float%20%28single-precision%29)))

(event MouseInput|EventActorOnClicked
  (params (ButtonPressed :type Key%20Structure))
  (CallFunction|Play))

(event EventDemonstrate
  (bind _out_animation (Variables|Default|GetOut%20Animation))
  (Class|ActorSequenceComponent|PlaySequence _out_animation)
  (EventDispatchers|AssignOnFinished (Variables|/Script/ActorSequence.ActorSequenceComponent|GetSequencePlayer _out_animation) (delegate Custom|OnFinished_Event)))

(event EventReset
  (Class|ActorSequenceComponent|StopSequence (Variables|Default|GetIn%20Animation))
  (Class|ActorSequenceComponent|StopSequence (Variables|Default|GetOut%20Animation))
  (Transformation|SetActorTransform (Variables|Default|GetStart%20Trans)))

(fn ConstructionScript)

(fn Play
  (if (Variables|Default|GetAnim%20Done?)
    (Utilities|FlowControl|Sequence
      (:then_0
        (if (Variables|Default|GetAnim%20Toogle)
          (Class|ActorSequenceComponent|PlaySequence (Variables|Default|GetOut%20Animation))
          (else
            (Class|ActorSequenceComponent|PlaySequence (Variables|Default|GetIn%20Animation)))))
      (:then_1
        (Variables|Default|SetAnim%20Toogle (not (Variables|Default|GetAnim%20Toogle)))))))