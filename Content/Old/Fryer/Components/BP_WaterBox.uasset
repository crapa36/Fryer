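; Interactive fryer water box actor that steps through an ordered list of slide in/out, cap open/close and fill/drain animations.
; Clicks or Excute play the next ActorSequence once the previous finishes, pausing at the last state until the wash button clears Ready.
; Designated ready and complete animations fire OnReady and OnCompleted callbacks.
; Demonstrate resets transforms and auto-chains sequences through finish bindings, stopping before the last state.
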(event Custom|OnFinished_Event
  (Variables|Default|SetAnim%20Done? true))

(event Custom|On%20Wash%20Button%20Clicked
  (if (Variables|Default|GetReady?)
    (Variables|Default|SetReady? false)
    (CallFunction|Play)))

(event Custom|HandleSequenceFinished
  (bind _anim (CallFunction|GetAnim (Variables|Default|GetIdx)))
  (EventDispatchers|UnbindEventfromOnFinished (Variables|/Script/ActorSequence.ActorSequenceComponent|GetSequencePlayer _anim) (EventDispatchers|CreateEvent :!event Custom|HandleSequenceFinished))
  (CallFunction|NextIdx)
  (CallFunction|PlayNextAnim))

(event Custom|PlayNextAnim
  (if (< (Variables|Default|GetIdx) (- (Utilities|Array|Length (Variables|Default|GetStates)) 1))
    (bind _anim (CallFunction|GetAnim (Variables|Default|GetIdx)))
    (Class|ActorSequenceComponent|PlaySequence _anim)
    (EventDispatchers|AssignOnFinished (Variables|/Script/ActorSequence.ActorSequenceComponent|GetSequencePlayer _anim) (EventDispatchers|CreateEvent :!event Custom|HandleSequenceFinished))))

(event Custom|Last%20Anim%20OnCompleted
  (Default|CallOnCompleted))

(event Custom|OnPlay_Event
  (Variables|Default|SetAnim%20Done? false))

(event Custom|Ready%20Anim%20OnCompleted
  (Default|CallOnReady))

(event EventBeginPlay
  (Variables|Default|SetBox%20Trans (Transformation|GetActorTransform))
  (Variables|Default|SetCap%20Trans (Transformation|GetRelativeTransform (Variables|Default|GetCap)))
  (Variables|Default|SetWater%20Trans (Transformation|GetRelativeTransform (Variables|Default|GetWater)))
  (Input|EnableInput (Game|GetPlayerController 0))
  (for _array_element (Actor|GetComponentsByClass "/Script/ActorSequence.ActorSequenceComponent")
    (EventDispatchers|AssignOnFinished (Variables|/Script/ActorSequence.ActorSequenceComponent|GetSequencePlayer _array_element) (delegate Custom|OnFinished_Event))
    (EventDispatchers|AssignOnPlay (Variables|/Script/ActorSequence.ActorSequenceComponent|GetSequencePlayer _array_element) (delegate Custom|OnPlay_Event)))
  (bind _anim (CallFunction|GetAnim (Utilities|Array|FindItem (Variables|Default|GetStates) (Variables|Default|GetComplete%20Anim))))
  (EventDispatchers|AssignOnFinished (Variables|/Script/ActorSequence.ActorSequenceComponent|GetSequencePlayer _anim) (delegate Custom|Last%20Anim%20OnCompleted))
  (bind _anim_2 (CallFunction|GetAnim (Utilities|Array|FindItem (Variables|Default|GetStates) (Variables|Default|GetReady%20Anim))))
  (EventDispatchers|AssignOnFinished (Variables|/Script/ActorSequence.ActorSequenceComponent|GetSequencePlayer _anim_2) (delegate Custom|Ready%20Anim%20OnCompleted)))

(event MouseInput|EventActorOnClicked
  (params (ButtonPressed :type Key%20Structure))
  (CallFunction|Play))

(event EventExcute
  (CallFunction|Play))

(event EventDemonstrate
  (CallFunction|Reset)
  (CallFunction|PlayNextAnim))

(event EventReset
  (bind _anim (CallFunction|GetAnim (Variables|Default|GetIdx)))
  (Class|ActorSequenceComponent|StopSequence _anim)
  (Variables|Default|SetIdx 0)
  (Variables|Default|SetAnim%20Done? true)
  (Variables|Default|SetReady? false)
  (Transformation|SetActorTransform (Variables|Default|GetBox%20Trans))
  (Transformation|SetRelativeTransform (Variables|Default|GetCap) (Variables|Default|GetCap%20Trans) false false)
  (Transformation|SetRelativeTransform (Variables|Default|GetWater) (Variables|Default|GetWater%20Trans) false false))

(fn ConstructionScript)

(fn Play
  (if (and (Variables|Default|GetAnim%20Done?) (not (Variables|Default|GetReady?)))
    (Utilities|FlowControl|Sequence
      (:then_0
        (bind _anim (CallFunction|GetAnim (Variables|Default|GetIdx)))
        (Class|ActorSequenceComponent|PlaySequence _anim))
      (:then_1
        (CallFunction|NextIdx)))))

(fn NextIdx
  (bind _states (Variables|Default|GetStates))
  (bind _returnvalue (Utilities|Array|Length _states))
  (if (not (Variables|Default|GetReady?))
    (bind _output_get (Variables|Default|SetIdx (Math|Integer|%(Integer) (+ (Variables|Default|GetIdx) 1) _returnvalue)))
    (if (== _output_get (- _returnvalue 1))
      (Variables|Default|SetReady? true))))

(fn GetAnim
  (params (Idx :type Integer))
  (switch string (Utilities|Array|Get(acopy) (Variables|Default|GetStates) Idx)
    (:Out
      (return (Variables|Default|GetOut%20Box)))
    (:In
      (return (Variables|Default|GetIn%20Box)))
    (:Fill
      (return (Variables|Default|GetFill%20Water)))
    (:Drain
      (return (Variables|Default|GetDrain%20Water)))
    (:Open
      (return (Variables|Default|GetOpen%20Cap)))
    (:Close
      (return (Variables|Default|GetClose%20Cap)))))