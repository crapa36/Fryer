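; Fryer Blueprint that coordinates washing and cooking through child actors for two buttons, clean and dirty water boxes, and a basket.
; Completing the wash button notifies both water boxes, while completing the cook button plays a looping sequence, guarded against replay until finished.
; Sequence end fires the cooking-completed dispatcher; Demonstrate bypasses the guard to play it directly.
; Reset messages all child actors, stops the sequence and restores the starting transform.
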(event Custom|OnFinished_Event
  (Variables|Default|SetAnim%20Done? true)
  (Default|CallOnCompletedCooking))

(event Custom|OnPlay_Event
  (Variables|Default|SetAnim%20Done? false))

(event Custom|Event%20Wash%20OnCompleted
  (Default|OnWashButtonClicked (Variables|Default|GetClean%20WaterBox%20Actor)))

(event Custom|Event%20Cook%20OnCompleted
  (CallFunction|PlayCookAnim))

(event EventBeginPlay
  (bind _cooking_anim (Variables|Default|GetCooking%20Anim))
  (bind _sequenceplayer (Variables|/Script/ActorSequence.ActorSequenceComponent|GetSequencePlayer _cooking_anim))
  (Variables|Default|SetStart%20Trans (Transformation|GetActorTransform))
  (CallFunction|CastChildActor)
  (EventDispatchers|AssignOnCompleted (Variables|Default|GetWashing%20Actor) (delegate Custom|Event%20Wash%20OnCompleted))
  (EventDispatchers|AssignOnCompleted (Variables|Default|GetCooking%20Actor) (delegate Custom|Event%20Cook%20OnCompleted))
  (EventDispatchers|AssignOnFinished _sequenceplayer (delegate Custom|OnFinished_Event))
  (EventDispatchers|AssignOnPlay _sequenceplayer (delegate Custom|OnPlay_Event)))

(event Collision|EventActorBeginOverlap
  (params (OtherActor :type Actor%20Object%20Reference)))

(event EventTick
  (params (DeltaSeconds :type Float%20%28single-precision%29)))

(event EventDemonstrate
  (Variables|Default|SetAnim%20Done? true)
  (CallFunction|PlayCookAnim))

(event EventReset
  (CallFunction|AllReset))

(fn ConstructionScript)

(fn CastChildActor
  (bind _asbp_water_box (Utilities|Casting|CastToBP_WaterBox (Variables|/Script/Engine.ChildActorComponent|GetChildActor (Variables|Default|GetCleanWaterBox)))
    (:then
      (Variables|Default|SetClean%20WaterBox%20Actor _asbp_water_box)
      (bind _asbp_water_box_2 (Utilities|Casting|CastToBP_WaterBox (Variables|/Script/Engine.ChildActorComponent|GetChildActor (Variables|Default|GetDirtyWaterBox))))
      (Variables|Default|SetDirty%20WaterBox%20Actor _asbp_water_box_2)
      (bind _asbp_basket (Utilities|Casting|CastToBP_Basket (Variables|/Script/Engine.ChildActorComponent|GetChildActor (Variables|Default|GetBasket))))
      (Variables|Default|SetBasket%20Actor _asbp_basket)
      (bind _asbp_button (Utilities|Casting|CastToBP_Button (Variables|/Script/Engine.ChildActorComponent|GetChildActor (Variables|Default|GetWashingButton))))
      (Variables|Default|SetWashing%20Actor _asbp_button)
      (bind _asbp_button_2 (Utilities|Casting|CastToBP_Button (Variables|/Script/Engine.ChildActorComponent|GetChildActor (Variables|Default|GetCookingButton))))
      (Variables|Default|SetCooking%20Actor _asbp_button_2))
    (:CastFailed
      _))
  (return))

(fn PlayCookAnim
  (if (Variables|Default|GetAnim%20Done?)
    (Class|MovieSceneSequencePlayer|PlayLooping (Variables|/Script/ActorSequence.ActorSequenceComponent|GetSequencePlayer (Variables|Default|GetCooking%20Anim)) 2)))

(fn AllReset
  (for _array_element (Actor|GetAllChildActors true)
    (Class|BPIExecutable|Reset(Message) _array_element)
    (Class|ActorSequenceComponent|StopSequence (Variables|Default|GetCooking%20Anim))
    (Transformation|SetActorTransform (Variables|Default|GetStart%20Trans))))