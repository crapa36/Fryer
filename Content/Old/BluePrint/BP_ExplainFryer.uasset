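; BP_ExplainFryer is an AI-controlled Fryer that steps through indexed explanations, paired with an on-screen explain UI.
; On BeginPlay it adds WBP_ExplainUI to the viewport, handing it a self reference, and publishes the starting index.
; NextExplain and PrevExplain move ExplainIndex within 0 to MaxIndex, then call NoticeIndex.
; NoticeIndex writes the index to the "Index" Blackboard key through ExplainFryerController.
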(event EventBeginPlay
  (|CallParentFunction)
  (bind _returnvalue (UserInterface|CreateWidget "/Game/Old/BluePrint/WBP_ExplainUI.WBP_ExplainUI_C" (Game|GetPlayerController 0) self))
  (bind _output_get (Variables|Default|SetExplain%20UI _returnvalue))
  (UserInterface|Viewport|AddtoViewport _output_get 0)
  (CallFunction|NoticeIndex))

(event Collision|EventActorBeginOverlap
  (params (OtherActor :type Actor%20Object%20Reference))
  (|CallParentFunction OtherActor) ; This node is disabled and will not be called.\nDrag off pins to build functionality.
)

(event EventTick
  (params (DeltaSeconds :type Float%20%28single-precision%29))
  (|CallParentFunction DeltaSeconds) ; This node is disabled and will not be called.\nDrag off pins to build functionality.
)

(fn ConstructionScript
  (|CallParentFunction))

(fn NextExplain
  (bind _result (Math|Integer|IncrementInt (Variables|Default|GetExplain%20Index))
    (:%20%20
      (Variables|Default|SetExplain%20Index (Math|Integer|Clamp(Integer) _result 0 (Variables|Default|GetMax%20Index)))
      (CallFunction|NoticeIndex))))

(fn PrevExplain
  (bind _result (Math|Integer|DecrementInt (Variables|Default|GetExplain%20Index))
    (:%20%20
      (Variables|Default|SetExplain%20Index (Math|Integer|Clamp(Integer) _result 0 (Variables|Default|GetMax%20Index)))
      (CallFunction|NoticeIndex))))

(fn NoticeIndex
  (bind _asexplain_fryer_controller (Utilities|Casting|CastToExplainFryerController (Pawn|GetController)))
  (Class|BlackboardComponent|SetValueasInt (AI|GetBlackboard _asexplain_fryer_controller) (Utilities|Name|MakeLiteralName "Index") (Variables|Default|GetExplain%20Index)))