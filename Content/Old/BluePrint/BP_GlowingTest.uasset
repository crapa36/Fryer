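; BP_GlowingTest is a test actor whose Cube toggles a glow when clicked.
; BeginPlay creates a dynamic material instance on the Cube and sets its glow color from the Glowing component.
; Clicks flip the Clickable component's state, which switches Glowing on or off.
; Tick polls Glowing and writes its amount, or zero when off, to the material's Intensity parameter.
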(event EventBeginPlay
  (bind _cube (Variables|Default|GetCube))
  (bind _returnvalue (Rendering|Material|CreateDynamicMaterialInstance _cube 0 (Rendering|Material|GetMaterial _cube 0) "None" :!class /Script/Engine.PrimitiveComponent))
  (bind _output_get (Variables|Default|SetGlowing%20Material _returnvalue))
  (Rendering|Material|SetVectorParameterValue _output_get "Glowing Color" (Variables|/Game/Old/BluePrint/BP_Glowing.BP_Glowing_C|GetColor (Variables|Default|GetGlowing)) :!class /Script/Engine.MaterialInstanceDynamic))

(event Collision|EventActorBeginOverlap
  (params (OtherActor :type Actor%20Object%20Reference)))

(event EventTick
  (params (DeltaSeconds :type Float%20%28single-precision%29))
  (bind _glowing (Variables|Default|GetGlowing))
  (if (Variables|/Game/Old/BluePrint/BP_Glowing.BP_Glowing_C|GetGlowing? _glowing)
    (Rendering|Material|SetScalarParameterValue (Variables|Default|GetGlowing%20Material) "Intensity" (Variables|/Game/Old/BluePrint/BP_Glowing.BP_Glowing_C|GetAmount _glowing) :!class /Script/Engine.MaterialInstanceDynamic)
    (else
      (Rendering|Material|SetScalarParameterValue (Variables|Default|GetGlowing%20Material) "Intensity" 0.0 :!class /Script/Engine.MaterialInstanceDynamic))))

(event MouseInput|EventActorOnClicked
  (params (ButtonPressed :type Key%20Structure))
  (bind _clickable (Variables|Default|GetClickable))
  (bind _glowing (Variables|Default|GetGlowing))
  (Default|ChangeState _clickable)
  (bind _newparam (Default|GetClicked _clickable))
  (if _newparam
    (Class|BPISwitchable|On(Message) _glowing)
    (else
      (Default|Off _glowing))))

(fn ConstructionScript)