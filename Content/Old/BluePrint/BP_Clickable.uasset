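; BP_Clickable is a small Blueprint that holds a Clicked boolean, apparently as a base for clickable objects.
; ClickRelease sets Clicked to true, Click sets it to false, and ChangeState toggles it.
; GetClicked returns the current value, while BeginPlay and Tick are disabled placeholders.
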(event EventBeginPlay)

(event EventTick
  (params (DeltaSeconds :type Float%20%28single-precision%29)))

(event EventClickRelease
  (Variables|Default|SetClicked? true))

(event EventClick
  (Variables|Default|SetClicked? false))

(event EventChangeState
  (if (Variables|Default|GetClicked?)
    (Variables|Default|SetClicked? false)
    (else
      (Variables|Default|SetClicked? true))))

(fn GetClicked
  (return (Variables|Default|GetClicked?)))