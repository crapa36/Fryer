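; BP_Level2_Pawn manages a set of Level 2 body actors and runs their execute animations one after another.
; On BeginPlay it gathers its BP_Level2_Body child actors into an array and registers itself as their Manager.
; CallExecute ignores requests while animating, issues resets on repeat runs, and starts at the first body.
; Each CallFinished advances to the next body, clearing the animating flag after the last.
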(event EventBeginPlay
  (for _array_element (Actor|GetAllChildActors true)
    (bind _asbp_level_2_body (Utilities|Casting|CastToBP_Level2_Body _array_element))
    (Utilities|Array|Add (Variables|Default|GetBodys) _asbp_level_2_body)
    (Variables|/Game/UtesPelare/Assets/Meshes/LMS/Level2/BP_Level2_Body.BP_Level2_Body_C|SetManager _asbp_level_2_body self)))

(event Collision|EventActorBeginOverlap
  (params (OtherActor :type Actor%20Object%20Reference)))

(event EventTick
  (params (DeltaSeconds :type Float%20%28single-precision%29)))

(event EventCallExecute
  (if (not (Variables|Default|GetAnimating))
    (Variables|Default|SetAnimating true)
    (if (Variables|Default|GetExecuted?)
      (for _array_element 0
        (Default|CallReset _array_element)
        (Variables|Default|SetExecuted? true)
        (Variables|Default|SetCurrentIndex 0)
        (Class|BPIAssemblyManager|CallExecute(Message) (Utilities|Array|Get(acopy) (Variables|Default|GetBodys) (Variables|Default|GetCurrentIndex))))
      (else
        (Variables|Default|SetExecuted? true)
        (Variables|Default|SetCurrentIndex 0)
        (Class|BPIAssemblyManager|CallExecute(Message) (Utilities|Array|Get(acopy) (Variables|Default|GetBodys) (Variables|Default|GetCurrentIndex)))))))

(event EventCallFinished
  (bind _result (Math|Integer|IncrementInt (Variables|Default|GetCurrentIndex))
    (:%20%20
      (if (< _result (Utilities|Array|Length (Variables|Default|GetBodys)))
        (Variables|Default|SetCurrentIndex _result)
        (Class|BPIAssemblyManager|CallExecute(Message) (Utilities|Array|Get(acopy) (Variables|Default|GetBodys) (Variables|Default|GetCurrentIndex)))
        (else
          (Variables|Default|SetAnimating false))))))

(fn ConstructionScript)