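; BP_Level1_Pawn is a Level 1 manager that triggers its child BP_Level1_Body actors one after another.
; On BeginPlay it collects all child BP_Level1_Body actors into an array and sets itself as their Manager.
; Execute starts the sequence unless one is already animating, calling ExecuteMessage on the first body.
; Each Finished event advances to the next body, clearing the Animating flag after the last.
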(event EventBeginPlay
  (for _array_element (Actor|GetAllChildActors true)
    (bind _asbp_level_1_body (Utilities|Casting|CastToBP_Level1_Body _array_element))
    (Utilities|Array|Add (Variables|Default|GetBodys) _asbp_level_1_body)
    (Variables|/Game/UtesPelare/Assets/Meshes/LMS/Level1/BP_Level1_Body.BP_Level1_Body_C|SetManager _asbp_level_1_body self)))

(event Collision|EventActorBeginOverlap
  (params (OtherActor :type Actor%20Object%20Reference)))

(event EventTick
  (params (DeltaSeconds :type Float%20%28single-precision%29)))

(event EventExecute
  (if (not (Variables|Default|GetAnimating))
    (Variables|Default|SetAnimating true)
    (Variables|Default|SetCurrentIndex 0)
    (Class|BPILegAssemblyManager|Execute(Message) (Utilities|Array|Get(acopy) (Variables|Default|GetBodys) (Variables|Default|GetCurrentIndex)))))

(event EventFinished
  (bind _result (Math|Integer|IncrementInt (Variables|Default|GetCurrentIndex))
    (:%20%20
      (if (< _result (Utilities|Array|Length (Variables|Default|GetBodys)))
        (Variables|Default|SetCurrentIndex _result)
        (Class|BPILegAssemblyManager|Execute(Message) (Utilities|Array|Get(acopy) (Variables|Default|GetBodys) (Variables|Default|GetCurrentIndex)))
        (else
          (Variables|Default|SetAnimating false))))))

(fn ConstructionScript)