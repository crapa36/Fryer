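; BP_LEVEL6 is the controller for step 6 of what appears to be a step-based manual, and serves as the view target while active.
; On BeginPlay it switches the player's view to itself, then sets the current step and binds sub-step button clicks to a blackboard "Sub Level" key through the ManualInstance game instance.
; Reset stops the CameraToMesh sequence, plays StartState and forwards a reset message to all child actors.
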(event EventBeginPlay
  (bind _returnvalue (Game|GetGameInstance))
  (bind _asmanual_instance (Utilities|Casting|CastToManualInstance _returnvalue))
  (Game|Player|SetViewTargetwithBlend (Game|GetPlayerController 0) self 0.0 "VTBlend_Linear" 0.0 false)
  (Default|SetNowStep _asmanual_instance 6 true)
  (Default|SetButtononClickedforSubStep _asmanual_instance (AI|GetBlackboard 0) "Sub Level" 2))

(event EventReset
  (Class|ActorSequenceComponent|StopSequence (Variables|Default|GetCamera%20To%20Mesh))
  (Class|ActorSequenceComponent|PlaySequence (Variables|Default|GetStart%20State))
  (for _array_element (Actor|GetAllChildActors true)
    (Class|BPIExecutable|Reset(Message) _array_element)))

(fn ConstructionScript)