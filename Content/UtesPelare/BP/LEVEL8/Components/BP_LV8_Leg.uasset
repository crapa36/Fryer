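; BP_LV8_Leg is a Level 8 leg component that spawns an alignment guide mesh on each of its sockets at BeginPlay.
; All guides are shadowless static meshes snapped to their socket and share one dynamic instance of M_Guide.
; The first guide's world height, lowered by a small offset, sets the material's "Z" parameter once.
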(event EventBeginPlay
  (CallFunction|SpawnGuide)
  (bind _returnvalue (Rendering|Material|GetScalarParameterValue (Variables|Default|GetDMI%20Guide) "Z" :!class /Script/Engine.MaterialInstanceDynamic)))

(fn ConstructionScript)

(fn SpawnGuide
  (bind _returnvalue (Rendering|Material|CreateDynamicMaterialInstance "/Game/UtesPelare/Assets/Meshes/KHI/M_Guide.M_Guide" "None" "None" :!class /Script/Engine.KismetMaterialLibrary))
  (Variables|Default|SetDMI%20Guide _returnvalue)
  (for _array_element (Transformation|GetAllSocketNames (Variables|Default|GetLeg))
    (bind _returnvalue_2 (AddComponent|AddStaticMeshComponent false))
    (Rendering|SetCastShadow _returnvalue_2 false)
    (Components|StaticMesh|SetStaticMesh _returnvalue_2 "/Game/UtesPelare/Assets/Meshes/KHI/SM_AlignmentGuide.SM_AlignmentGuide")
    (Rendering|Material|SetMaterial _returnvalue_2 0 (Variables|Default|GetDMI%20Guide))
    (Transformation|AttachComponentToComponent _returnvalue_2 (Variables|Default|GetLeg) _array_element "SnapToTarget" "SnapToTarget" "SnapToTarget" true)
    (Utilities|FlowControl|DoOnce false
      (:Completed
        (Rendering|Material|SetScalarParameterValue (Variables|Default|GetDMI%20Guide) "Z" (- (.z (Transformation|GetWorldLocation _returnvalue_2)) 2.0) :!class /Script/Engine.MaterialInstanceDynamic)))))