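; Level 8 step actor that lets the player choose a default or turned table shape and acts as the view target.
; MoveSelectView creates a second player to show both child-actor models in separate views alongside the WBP_Select buttons.
; A choice is stored in ManualInstance, then OnSelected removes that player, restores the view, sets the blackboard SubLevel and orients the tabletop and target hole.
; StopAnim jumps the LegDown and CameraMove sequence playback.
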(event Custom|Move%20Select%20View
  (Widget|SetVisibility (Variables|/Game/UtesPelare/Widget/ExplainWBP.ExplainWBP_C|GetNextButton (Variables|/Game/UtesPelare/BluePrints/sh/ManualInstance.ManualInstance_C|GetExplain%20UI (Variables|Default|GetInstance))) "Hidden")
  (Widget|SetVisibility (Variables|Default|GetSelect%20UI) "Visible")
  (Class|GameplayStatics|CreatePlayer 1)
  (Game|Player|SetViewTargetwithBlend (Game|GetPlayerController 0) (Variables|/Script/Engine.ChildActorComponent|GetChildActor (Variables|Default|GetDefault%20Model)) 0.0 "VTBlend_Linear" 0.0 false)
  (Game|Player|SetViewTargetwithBlend (Game|GetPlayerController 1) (Variables|/Script/Engine.ChildActorComponent|GetChildActor (Variables|Default|GetTurn%20Model)) 0.0 "VTBlend_Linear" 0.0 false))

(event Custom|Default%20OnClicked_Event
  (Variables|/Game/UtesPelare/BluePrints/sh/ManualInstance.ManualInstance_C|SetDefault%20Shape? (Variables|Default|GetInstance) true)
  (Default|CallOnSelected))

(event Custom|On%20Selected_Event
  (bind _table_target_hole (Variables|Default|GetTable%20Target%20Hole))
  (bind _tabletop (Variables|Default|GetTableTop))
  (Class|GameplayStatics|RemovePlayer (Game|GetPlayerController 1) false)
  (Widget|SetVisibility (Variables|Default|GetSelect%20UI) "Hidden")
  (Game|Player|SetViewTargetwithBlend (Game|GetPlayerController 0) self 0.0 "VTBlend_Linear" 0.0 false)
  (Class|BlackboardComponent|SetValueasInt (AI|GetBlackboard 0) (Utilities|Name|MakeLiteralName "SubLevel") 1)
  (Widget|SetVisibility (Variables|/Game/UtesPelare/Widget/ExplainWBP.ExplainWBP_C|GetNextButton (Variables|/Game/UtesPelare/BluePrints/sh/ManualInstance.ManualInstance_C|GetExplain%20UI (Variables|Default|GetInstance))) "Visible")
  (Default|SetSubStepText (Variables|Default|GetInstance) 1)
  (if (Variables|/Game/UtesPelare/BluePrints/sh/ManualInstance.ManualInstance_C|GetDefault%20Shape? (Variables|Default|GetInstance))
    (Transformation|SetRelativeRotation _tabletop "0, 0, 0" false false)
    (Transformation|SetRelativeLocation _table_target_hole "0.000000,-16.000000,1.900000" false false)
    (else
      (Transformation|SetRelativeRotation _tabletop "0.000000,180.000000,0.000000" false false)
      (Transformation|SetRelativeLocation _table_target_hole "0.000000,12.500000,1.900000" false false))))

(event Custom|Bindind%20for%20Select
  (EventDispatchers|AssignOnClicked (Variables|/Game/UtesPelare/BP/LEVEL8/WBP_Select.WBP_Select_C|GetDefaultButton (Variables|Default|GetSelect%20UI)) (delegate Custom|Default%20OnClicked_Event))
  (EventDispatchers|AssignOnClicked (Variables|/Game/UtesPelare/BP/LEVEL8/WBP_Select.WBP_Select_C|GetTurnButton (Variables|Default|GetSelect%20UI)) (delegate Custom|Turn%20OnClicked_Event)))

(event Custom|Turn%20OnClicked_Event
  (Variables|/Game/UtesPelare/BluePrints/sh/ManualInstance.ManualInstance_C|SetDefault%20Shape? (Variables|Default|GetInstance) false)
  (Default|CallOnSelected))

(event EventBeginPlay
  (Game|Player|SetViewTargetwithBlend (Game|GetPlayerController 0) self 0.0 "VTBlend_Linear" 0.0 false)
  (bind _returnvalue (UserInterface|CreateWidget "/Game/UtesPelare/BP/LEVEL8/WBP_Select.WBP_Select_C"))
  (bind _aswbp_select (Utilities|Casting|CastToWBP_Select _returnvalue))
  (bind _output_get (Variables|Default|SetSelect%20UI _aswbp_select))
  (UserInterface|Viewport|AddtoViewport _output_get 0)
  (Widget|SetVisibility _output_get "Hidden")
  (bind _asmanual_instance (Utilities|Casting|CastToManualInstance (Game|GetGameInstance)))
  (Variables|Default|SetInstance _asmanual_instance)
  (EventDispatchers|BindEventtoOnSelected (delegate Custom|On%20Selected_Event))
  (CallFunction|BindindforSelect)
  (Default|SetButtononClickedforSubStep (Variables|Default|GetInstance) (AI|GetBlackboard 0) "SubLevel" 1))

(event Collision|EventActorBeginOverlap
  (params (OtherActor :type Actor%20Object%20Reference)))

(event EventTick
  (params (DeltaSeconds :type Float%20%28single-precision%29)))

(fn ConstructionScript)

(fn StopAnim
  (Components|Timeline|SetPlaybackPosition (Variables|/Script/ActorSequence.ActorSequenceComponent|GetSequencePlayer (Variables|Default|GetLeg%20Down)) (Utilities|Struct|MakeMovieSceneSequencePlaybackParams "(FrameNumber=(Value=0),SubFrame=0.000000)" 0.0 "" "(Hours=0,Minutes=0,Seconds=0,Frames=0,Subframe=0.000000,bDropFrameFormat=False)" "Frame" "Jump" true))
  (Components|Timeline|SetPlaybackPosition (Variables|/Script/ActorSequence.ActorSequenceComponent|GetSequencePlayer (Variables|Default|GetCamera%20Move)) (Utilities|Struct|MakeMovieSceneSequencePlaybackParams "(FrameNumber=(Value=0),SubFrame=0.000000)" 0.0 "" "(Hours=0,Minutes=0,Seconds=0,Frames=0,Subframe=0.000000,bDropFrameFormat=False)" "Frame" "Jump" true)))