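; Level 5 actor that acts as the player's camera view target and handles that level's sub-step setup and reset.
; On BeginPlay it blends the view to itself and has ManualInstance wire the sub-step button to its blackboard's "Sub Level" key, capped at 2.
; Reset stops the CameraMove and CameraWalking sequences, plays StartState, and sends ResetMessage to all child actors, including nested ones.
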(event EventBeginPlay
  ;[0.15 0.15 0.15 0.5] 카메라 변경
  (CallFunction|InitFunc))

(event Collision|EventActorBeginOverlap
  (params (OtherActor :type Actor%20Object%20Reference)))

(event EventTick
  (params (DeltaSeconds :type Float%20%28single-precision%29)))

(event EventReset
  (Class|ActorSequenceComponent|StopSequence (Variables|Default|GetCamera%20Move))
  (Class|ActorSequenceComponent|StopSequence (Variables|Default|GetCamera%20Walking))
  (Class|ActorSequenceComponent|PlaySequence (Variables|Default|GetStart%20State))
  (for _array_element (Actor|GetAllChildActors true)
    (Class|BPIExecutable|Reset(Message) _array_element)))

(event EventDestroyed
  ;[0.15 0.15 0.15 0.5] Not Require
)

(event EventEndPlay
  (params (EndPlayReason :type EEndPlayReason%20Enum :default "Destroyed"))
  ;[0.15 0.15 0.15 0.5] Not Require
)

(fn ConstructionScript)

(fn InitFunc
  (Game|Player|SetViewTargetwithBlend (Game|GetPlayerController 0) self 0.0 "VTBlend_Linear" 0.0 false)
  (Default|SetButtononClickedforSubStep (.AsManual%20Instance (Utilities|Casting|CastToManualInstance (Game|GetGameInstance))) (AI|GetBlackboard 0) "Sub Level" 2))