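; Level 10 pawn of an interactive assembly manual, showing hooks and bolts being fitted to a table.
; It takes the camera, orients the tabletop, spawns BP_LV10_Hook pairs at mesh sockets and plays their spawn sequences.
; It then spawns AIC_LV10 to possess itself, with bracket keys switching the blackboard SubLevel.
; Bolt events play, replay or skip hook tightening sequences, signalling completion through CallOnCompleted, as does the camera sequence.
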(event Custom|OnFinished_Event
  (Default|CallOnCompleted))

(event EventBeginPlay
  (Game|Player|SetViewTargetwithBlend (Game|GetPlayerController 0) self 0.0 "VTBlend_Linear" 0.0 false)
  (EventDispatchers|AssignOnFinished (Variables|/Script/ActorSequence.ActorSequenceComponent|GetSequencePlayer (Variables|Default|GetMove%20Camera)) (delegate Custom|OnFinished_Event))
  (bind _output_get (Variables|Default|SetInstance (.AsManual%20Instance (Utilities|Casting|CastToManualInstance (Game|GetGameInstance)))))
  (Default|SetTextUI _output_get)
  (CallFunction|SpawnHooks)
  (CallFunction|SetTableShape)
  (CallFunction|AssembleComponents))

(event Collision|EventActorBeginOverlap
  (params (OtherActor :type Actor%20Object%20Reference)))

(event EventTick
  (params (DeltaSeconds :type Float%20%28single-precision%29)))

(event Input|KeyboardEvents|RightBracket
  (params (Key :type Key%20Structure :default "None"))
  (:Pressed
    (Class|BlackboardComponent|SetValueasInt (AI|GetBlackboard 0) (Utilities|Name|MakeLiteralName "SubLevel") 1)))

(event Input|KeyboardEvents|LeftBracket
  (params (Key :type Key%20Structure :default "None"))
  (:Pressed
    (Class|BlackboardComponent|SetValueasInt (AI|GetBlackboard 0) (Utilities|Name|MakeLiteralName "SubLevel"))))

(event Custom|Assemble%20Components
  (EventDispatchers|AssignOnFinished (Variables|/Script/ActorSequence.ActorSequenceComponent|GetSequencePlayer (Variables|/Game/UtesPelare/BP/LEVEL10/Components/BP_LV10_Hook.BP_LV10_Hook_C|GetSpawn%20Effect (Utilities|Array|Get(acopy) (Variables|Default|GetHooks)))) (delegate Custom|Hook%20OnFinished_Event))
  (for _array_element (Variables|Default|GetHooks)
    (Sequencer|Player|Play (Variables|/Script/ActorSequence.ActorSequenceComponent|GetSequencePlayer (Variables|/Game/UtesPelare/BP/LEVEL10/Components/BP_LV10_Hook.BP_LV10_Hook_C|GetSpawn%20Effect _array_element)) :!class /Script/MovieScene.MovieSceneSequencePlayer)))

(event Custom|Reset%20Bolts
  (params (begin :type Integer) (end :type Integer))
  (bind _returnvalue (- end 1))
  (CallFunction|BindComplete (* _returnvalue 2))
  (for _index (range begin _returnvalue)
    (for _index_2 (range 0 1)
      (Sequencer|Player|Stop (Variables|/Script/ActorSequence.ActorSequenceComponent|GetSequencePlayer (Variables|/Game/UtesPelare/BP/LEVEL10/Components/BP_LV10_Hook.BP_LV10_Hook_C|GetTight (Utilities|Array|Get(acopy) (Variables|Default|GetHooks) (+ (* _index 2) _index_2)))) :!class /Script/MovieScene.MovieSceneSequencePlayer)
      (Sequencer|Player|Play (Variables|/Script/ActorSequence.ActorSequenceComponent|GetSequencePlayer (Variables|/Game/UtesPelare/BP/LEVEL10/Components/BP_LV10_Hook.BP_LV10_Hook_C|GetTight (Utilities|Array|Get(acopy) (Variables|Default|GetHooks) (+ (* _index 2) _index_2)))) :!class /Script/MovieScene.MovieSceneSequencePlayer)
      (Class|MovieSceneSequencePlayer|Playto (Variables|/Script/ActorSequence.ActorSequenceComponent|GetSequencePlayer (Variables|/Game/UtesPelare/BP/LEVEL10/Components/BP_LV10_Hook.BP_LV10_Hook_C|GetTight (Utilities|Array|Get(acopy) (Variables|Default|GetHooks) (+ (* _index 2) _index_2))))))))

(event Custom|Bind%20Complete
  (params (idx :type Integer))
  (bind _hooks (Variables|Default|GetHooks))
  (bind _output (Utilities|Array|Get(acopy) _hooks idx))
  (bind _tight (Variables|/Game/UtesPelare/BP/LEVEL10/Components/BP_LV10_Hook.BP_LV10_Hook_C|GetTight _output))
  (bind _sequenceplayer (Variables|/Script/ActorSequence.ActorSequenceComponent|GetSequencePlayer _tight))
  (EventDispatchers|BindEventtoOnPause _sequenceplayer (delegate Custom|CustomEvent_1))
  (EventDispatchers|BindEventtoOnStop _sequenceplayer (delegate Custom|CustomEvent_1))
  (EventDispatchers|AssignOnFinished _sequenceplayer (delegate Custom|CustomEvent_1)))

(event Custom|CustomEvent_1
  (EventDispatchers|UnbindEventfromOnPause (Variables|/Script/ActorSequence.ActorSequenceComponent|GetSequencePlayer (Variables|/Game/UtesPelare/BP/LEVEL10/Components/BP_LV10_Hook.BP_LV10_Hook_C|GetTight (Utilities|Array|Get(acopy) (Variables|Default|GetHooks) (stale Custom|Bind%20Complete idx)))) (delegate Custom|CustomEvent_1))
  (EventDispatchers|UnbindEventfromOnStop (Variables|/Script/ActorSequence.ActorSequenceComponent|GetSequencePlayer (Variables|/Game/UtesPelare/BP/LEVEL10/Components/BP_LV10_Hook.BP_LV10_Hook_C|GetTight (Utilities|Array|Get(acopy) (Variables|Default|GetHooks) (stale Custom|Bind%20Complete idx)))) (delegate Custom|CustomEvent_1))
  (EventDispatchers|UnbindEventfromOnFinished (Variables|/Script/ActorSequence.ActorSequenceComponent|GetSequencePlayer (Variables|/Game/UtesPelare/BP/LEVEL10/Components/BP_LV10_Hook.BP_LV10_Hook_C|GetTight (Utilities|Array|Get(acopy) (Variables|Default|GetHooks) (stale Custom|Bind%20Complete idx)))) (delegate Custom|CustomEvent_1))
  (Default|CallOnCompleted))

(event Custom|Hook%20OnFinished_Event
  (EventDispatchers|UnbindEventfromOnFinished (Variables|/Script/ActorSequence.ActorSequenceComponent|GetSequencePlayer (Variables|/Game/UtesPelare/BP/LEVEL10/Components/BP_LV10_Hook.BP_LV10_Hook_C|GetSpawn%20Effect (Utilities|Array|Get(acopy) (Variables|Default|GetHooks)))) (delegate Custom|Hook%20OnFinished_Event))
  (bind _returnvalue (Game|SpawnActorfromClass "/Game/UtesPelare/BP/LEVEL10/AI/AIC_LV10.AIC_LV10_C" (Math|Transform|MakeTransform "0, 0, 0") "Undefined" "MultiplyWithRoot" 0 0))
  (Pawn|Possess _returnvalue self))

(event Custom|Tight%20Bolts
  (params (begin :type Integer) (end :type Integer))
  (bind _returnvalue (- end 1))
  (CallFunction|BindComplete (* _returnvalue 2))
  (for _index (range begin _returnvalue)
    (for _index_2 (range 0 1)
      (Class|ActorSequenceComponent|PlaySequence (Variables|/Game/UtesPelare/BP/LEVEL10/Components/BP_LV10_Hook.BP_LV10_Hook_C|GetTight (Utilities|Array|Get(acopy) (Variables|Default|GetHooks) (+ (* _index 2) _index_2)))))))

(event Custom|Set%20Complete%20Bolts
  (for _index (range 0 1)
    (Sequencer|Player|Play (Variables|/Script/ActorSequence.ActorSequenceComponent|GetSequencePlayer (Variables|/Game/UtesPelare/BP/LEVEL10/Components/BP_LV10_Hook.BP_LV10_Hook_C|GetTight (Utilities|Array|Get(acopy) (Variables|Default|GetHooks) _index))) :!class /Script/MovieScene.MovieSceneSequencePlayer)
    (Class|MovieSceneSequencePlayer|GotoEndandStop (Variables|/Script/ActorSequence.ActorSequenceComponent|GetSequencePlayer (Variables|/Game/UtesPelare/BP/LEVEL10/Components/BP_LV10_Hook.BP_LV10_Hook_C|GetTight (Utilities|Array|Get(acopy) (Variables|Default|GetHooks) _index)))))
  (Default|CallOnCompleted))

(fn ConstructionScript)

(fn SpawnHooks
  (bind _meshtop (Variables|Default|GetMeshTop))
  (bind _returnvalue (Transformation|GetAllSocketNames _meshtop))
  (for (_array_element _array_index) _returnvalue
    (for _index (range 0 1)
      (bind _returnvalue_2 (AddComponent|AddChildActorComponent false (Transformation|GetSocketTransform (Variables|Default|GetMeshTop) _array_element "RTS_Actor")))
      (ChildActorComponent|SetChildActorClass _returnvalue_2 "/Game/UtesPelare/BP/LEVEL10/Components/BP_LV10_Hook.BP_LV10_Hook_C")
      (bind _asbp_lv10_hook (Utilities|Casting|CastToBP_LV10_Hook (Variables|/Script/Engine.ChildActorComponent|GetChildActor _returnvalue_2)))
      (Utilities|Array|Add (Variables|Default|GetHooks) _asbp_lv10_hook)
      (Utilities|FlowControl|FlipFlop
        (:A
          (if (== _array_index (Utilities|Array|LastIndex _returnvalue))
            (Transformation|AddRelativeRotation _returnvalue_2 "0.000000,-90.000000,0.000000" false false)
            (Transformation|AddRelativeRotation (Variables|/Game/UtesPelare/BP/LEVEL10/Components/BP_LV10_Hook.BP_LV10_Hook_C|GetHook _asbp_lv10_hook) "0.000000,90.000000,0.000000" false false)))
        (:B
          (Transformation|AddLocalOffset _returnvalue_2 "-9.000000,0.000000,0.000000" false false)
          (if (== _array_index (Utilities|Array|LastIndex _returnvalue))
            (Transformation|AddRelativeRotation _returnvalue_2 "0.000000,180.000000,0.000000" false false)
            (else
              (Transformation|AddRelativeRotation _returnvalue_2 "0.000000,90.000000,0.000000" false false)
              (Transformation|SetRelativeRotation (Variables|/Game/UtesPelare/BP/LEVEL10/Components/BP_LV10_Hook.BP_LV10_Hook_C|GetHook _asbp_lv10_hook) "0.000000,90.000000,0.000000" false false)))))))
  (for _index_2 (range 0 1)
    _))

(fn SetTableShape
  (bind _asmanual_instance (Utilities|Casting|CastToManualInstance (Game|GetGameInstance)))
  (bind _output_get (Variables|Default|SetInstance _asmanual_instance))
  (if (not (Variables|/Game/UtesPelare/BluePrints/sh/ManualInstance.ManualInstance_C|GetDefault%20Shape? _output_get))
    (Transformation|SetRelativeRotation (Variables|Default|GetTableTop) "0.000000,180.000000,0.000000" false false)))