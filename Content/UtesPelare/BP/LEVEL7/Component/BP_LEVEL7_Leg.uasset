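; BP_LEVEL7_Leg is a Level 7 leg component actor that runs its child bolt actors in a named sequence.
; BeginPlay gathers the BP_LEVEL7_Bolt1 child actors, and Excute resets, binds to their completion events and starts Anim.
; Each Anim call executes the bolt matching the next entry in Names, then rewinds the index and fires OnCompeleted after the last.
; Reset forwards a reset message to every bolt.
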(event Custom|OnCompeleted_Event
  (EventDispatchers|UnbindEventfromOnCompeleted (stale EventExcute _array_element) (EventDispatchers|CreateEvent :!event Custom|CustomEvent))
  (Development|PrintString "Hi"))

(event Custom|CustomEvent
  (CallFunction|Anim))

(event EventBeginPlay
  (for _array_element (Actor|GetAllChildActors true)
    (bind _asbp_level7_bolt_1 (Utilities|Casting|CastToBP_LEVEL7_Bolt1 _array_element))
    (Utilities|Array|Add (Variables|Default|GetBolts) _asbp_level7_bolt_1)))

(event Collision|EventActorBeginOverlap
  (params (OtherActor :type Actor%20Object%20Reference)))

(event EventTick
  (params (DeltaSeconds :type Float%20%28single-precision%29)))

(event EventExcute
  (Class|BPIExcutable|Reset(Message) self)
  (for _array_element (Variables|Default|GetBolts)
    (EventDispatchers|AssignOnCompeleted _array_element (EventDispatchers|CreateEvent :!event Custom|CustomEvent)))
  (EventDispatchers|AssignOnCompeleted (delegate Custom|OnCompeleted_Event))
  (CallFunction|Anim))

(event EventReset
  (for _array_element (Variables|Default|GetBolts)
    (Class|BPIExcutable|Reset(Message) _array_element)))

(fn ConstructionScript
  (|CallParentFunction))

(fn Anim
  (if (< (+ (Variables|Default|GetIdx) 1) (Utilities|Array|Length (Variables|Default|GetNames)))
    (Variables|Default|SetIdx (+ (Variables|Default|GetIdx) 1))
    (for _array_element (Variables|Default|GetBolts)
      (if (== (Variables|/Game/UtesPelare/BP/LEVEL7/Component/BP_LEVEL7_Bolt1.BP_LEVEL7_Bolt1_C|GetName _array_element) (Utilities|Array|Get(acopy) (Variables|Default|GetNames) (Variables|Default|GetIdx)))
        (Class|BPIExcutable|Excute(Message) _array_element)
        (return)))
    (else
      (Variables|Default|SetIdx -1)
      (Development|PrintString "Hello")
      (Default|CallOnCompeleted))))