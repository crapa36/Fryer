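; Clickable Level 7 bolt step that plays tightening sequences and signals completion when each one finishes.
; Execute loops a highlight sequence; clicking the box or calling Demonstrate plays it with zero loops, so its finish event triggers tightening.
; The Half flag selects a single full-tighten pass or toggling between half-tight and half-to-full passes.
; Reset stops all sequences, restores the start state and clears click and toggle flags.
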(event OnClicked(Box)
  (params (TouchedComponent :type Primitive%20Component%20Object%20Reference) (ButtonPressed :type Key%20Structure :default "None"))
  (if (Variables|Default|GetClickable)
    (Variables|Default|SetClickable false)
    (CallFunction|StopHighLight)))

(event Custom|OnFinished_Event
  (Class|ActorSequenceComponent|PlaySequence (Variables|Default|GetFull%20Tight)))

(event Custom|CustomEvent
  (Default|CallOnCompeleted))

(event Custom|OnFinished_Event_0
  (Variables|Default|SetTogle (not (Variables|Default|GetTogle)))
  (if (Variables|Default|GetTogle)
    (Class|ActorSequenceComponent|PlaySequence (Variables|Default|GetHalf%20Tight))
    (else
      (Class|ActorSequenceComponent|PlaySequence (Variables|Default|GetHalf%20to%20Full%20Tight)))))

(event EventBeginPlay
  (bind _highlight (Variables|Default|GetHighlight))
  (bind _sequenceplayer (Variables|/Script/ActorSequence.ActorSequenceComponent|GetSequencePlayer _highlight))
  (EventDispatchers|AssignOnFinished (Variables|/Script/ActorSequence.ActorSequenceComponent|GetSequencePlayer (Variables|Default|GetHalf%20to%20Full%20Tight)) (delegate Custom|CustomEvent))
  (EventDispatchers|AssignOnFinished (Variables|/Script/ActorSequence.ActorSequenceComponent|GetSequencePlayer (Variables|Default|GetFull%20Tight)) (delegate Custom|CustomEvent))
  (EventDispatchers|AssignOnFinished (Variables|/Script/ActorSequence.ActorSequenceComponent|GetSequencePlayer (Variables|Default|GetHalf%20Tight)) (delegate Custom|CustomEvent))
  (if (Variables|Default|GetHalf?)
    (EventDispatchers|AssignOnFinished _sequenceplayer (delegate Custom|OnFinished_Event))
    (else
      (EventDispatchers|AssignOnFinished _sequenceplayer (delegate Custom|OnFinished_Event_0)))))

(event EventTick
  (params (DeltaSeconds :type Float%20%28single-precision%29)))

(event EventExecute
  (CallFunction|HighLighting))

(event EventDemonstrate
  (CallFunction|PlayAnim))

(event EventReset
  (CallFunction|StopAnim)
  (Variables|Default|SetClickable false)
  (Variables|Default|SetTogle false))

(fn ConstructionScript
  (|CallParentFunction))

(fn StopAnim
  (Class|ActorSequenceComponent|StopSequence (Variables|Default|GetHalf%20Tight))
  (Class|ActorSequenceComponent|StopSequence (Variables|Default|GetHalf%20to%20Full%20Tight))
  (Class|ActorSequenceComponent|StopSequence (Variables|Default|GetFull%20Tight))
  (Class|ActorSequenceComponent|StopSequence (Variables|Default|GetHighlight))
  (Class|ActorSequenceComponent|PlaySequence (Variables|Default|GetStart%20State)))

(fn StopHighLight
  (Class|MovieSceneSequencePlayer|PlayLooping (Variables|/Script/ActorSequence.ActorSequenceComponent|GetSequencePlayer (Variables|Default|GetHighlight)) 0))

(fn HighLighting
  (Class|MovieSceneSequencePlayer|PlayLooping (Variables|/Script/ActorSequence.ActorSequenceComponent|GetSequencePlayer (Variables|Default|GetHighlight)) -1))

(fn PlayAnim
  (Class|MovieSceneSequencePlayer|PlayLooping (Variables|/Script/ActorSequence.ActorSequenceComponent|GetSequencePlayer (Variables|Default|GetHighlight)) 0))