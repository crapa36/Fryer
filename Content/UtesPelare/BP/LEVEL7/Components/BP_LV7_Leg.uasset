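; BP_LV7_Leg is a Level 7 leg actor that runs its bolts one at a time in a named order.
; On BeginPlay it collects its BP_LV7_Bolt1 child actors.
; Execute and Demonstrate bind to each bolt's completion and start Anim, which messages the bolt matching the next entry in Names to execute or demonstrate.
; When the list is exhausted, it resets the index and fires its own completion dispatcher.
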(event Custom|AnimEvent
  (CallFunction|Anim))

(event EventBeginPlay
  (for _array_element (Actor|GetAllChildActors true)
    (bind _asbp_lv7_bolt_1 (Utilities|Casting|CastToBP_LV7_Bolt1 _array_element))
    (Utilities|Array|Add (Variables|Default|GetBolts) _asbp_lv7_bolt_1)))

(event Collision|EventActorBeginOverlap
  (params (OtherActor :type Actor%20Object%20Reference)))

(event EventTick
  (params (DeltaSeconds :type Float%20%28single-precision%29)))

(event EventReset
  (Development|PrintString "RESET")
  (Variables|Default|SetIdx -1)
  (for _array_element (Variables|Default|GetBolts)
    (Class|BPIExecutable|Reset(Message) _array_element)))

(event EventDemonstrate
  (Variables|Default|SetDemo? true)
  (CallFunction|Reset)
  (for _array_element (Variables|Default|GetBolts)
    (EventDispatchers|AssignOnCompeleted _array_element (EventDispatchers|CreateEvent :!event Custom|AnimEvent)))
  (CallFunction|Anim))

(event EventExecute
  (Variables|Default|SetDemo? false)
  (for _array_element (Variables|Default|GetBolts)
    (EventDispatchers|AssignOnCompeleted _array_element (EventDispatchers|CreateEvent :!event Custom|AnimEvent)))
  (CallFunction|Anim))

(fn ConstructionScript
  (|CallParentFunction))

(fn Anim
  (if (< (+ (Variables|Default|GetIdx) 1) (Utilities|Array|Length (Variables|Default|GetNames)))
    (Variables|Default|SetIdx (+ (Variables|Default|GetIdx) 1))
    (for _array_element (Variables|Default|GetBolts)
      (if (== (Variables|/Game/UtesPelare/BP/LEVEL7/Components/BP_LV7_Bolt1.BP_LV7_Bolt1_C|GetName _array_element) (Utilities|Array|Get(acopy) (Variables|Default|GetNames) (Variables|Default|GetIdx)))
        (if (Variables|Default|GetDemo?)
          (Class|BPIExecutable|Demonstrate(Message) _array_element)
          (else
            (Class|BPIExecutable|Execute(Message) _array_element)))
        (return)))
    (else
      (Variables|Default|SetIdx -1)
      (Default|CallOnCompeleted))))