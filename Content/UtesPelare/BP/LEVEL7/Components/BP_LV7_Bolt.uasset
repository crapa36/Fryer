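; Level 7 bolt actor that plays highlight and tightening sequences, with a number widget kept just above it.
; When the highlight finishes, the Half flag selects either a full tighten or a toggle between half and half-to-full stages.
; Tightening sequences report completion when finished.
; Reset, SetHalf, SetOrign and SetComplete stop playback and snap the bolt to start, half or complete states.
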(event Custom|OnFinished_Event
  (Class|ActorSequenceComponent|PlaySequence (Variables|Default|GetFull%20Tight)))

(event Custom|Event%20Set%20Orign
  (CallFunction|StopAnim)
  (Class|ActorSequenceComponent|PlaySequence (Variables|Default|GetStart%20State))
  (Variables|Default|SetToggle false))

(event Custom|CustomEvent
  (Default|CallOnCompleted))

(event Custom|Event%20Set%20Half
  (bind _half_tight (Variables|Default|GetHalf%20Tight))
  (bind _sequenceplayer (Variables|/Script/ActorSequence.ActorSequenceComponent|GetSequencePlayer _half_tight))
  (CallFunction|StopAnim)
  (Sequencer|Player|Play _sequenceplayer :!class /Script/MovieScene.MovieSceneSequencePlayer)
  (Class|MovieSceneSequencePlayer|GotoEndandStop _sequenceplayer)
  (Class|ActorSequenceComponent|PlaySequence (Variables|Default|GetHide%20Circular%20Arrow))
  (Variables|Default|SetToggle true))

(event Custom|OnFinished_Event_0
  (Variables|Default|SetToggle (not (Variables|Default|GetToggle)))
  (if (Variables|Default|GetToggle)
    (Class|ActorSequenceComponent|PlaySequence (Variables|Default|GetHalf%20Tight))
    (else
      (Class|ActorSequenceComponent|PlaySequence (Variables|Default|GetHalf%20to%20Full%20Tight)))))

(event Custom|Event%20Set%20Complete
  (bind _half_to_full_tight (Variables|Default|GetHalf%20to%20Full%20Tight))
  (bind _sequenceplayer (Variables|/Script/ActorSequence.ActorSequenceComponent|GetSequencePlayer _half_to_full_tight))
  (CallFunction|StopAnim)
  (Sequencer|Player|Play _sequenceplayer :!class /Script/MovieScene.MovieSceneSequencePlayer)
  (Class|MovieSceneSequencePlayer|GotoEndandStop _sequenceplayer)
  (Variables|Default|SetToggle false))

(event EventBeginPlay
  (bind _highlight (Variables|Default|GetHighlight))
  (bind _sequenceplayer (Variables|/Script/ActorSequence.ActorSequenceComponent|GetSequencePlayer _highlight))
  (Variables|Default|SetNumber%20Text (.AsWBP%20LV7%20Number (Utilities|Casting|CastToWBP_LV7_Number (UserInterface|GetWidget (Variables|Default|GetNum)))))
  (EventDispatchers|AssignOnFinished (Variables|/Script/ActorSequence.ActorSequenceComponent|GetSequencePlayer (Variables|Default|GetHalf%20to%20Full%20Tight)) (delegate Custom|CustomEvent))
  (EventDispatchers|AssignOnFinished (Variables|/Script/ActorSequence.ActorSequenceComponent|GetSequencePlayer (Variables|Default|GetFull%20Tight)) (delegate Custom|CustomEvent))
  (EventDispatchers|AssignOnFinished (Variables|/Script/ActorSequence.ActorSequenceComponent|GetSequencePlayer (Variables|Default|GetHalf%20Tight)) (delegate Custom|CustomEvent))
  (if (Variables|Default|GetHalf?)
    (EventDispatchers|AssignOnFinished _sequenceplayer (delegate Custom|OnFinished_Event))
    (else
      (EventDispatchers|AssignOnFinished _sequenceplayer (delegate Custom|OnFinished_Event_0)))))

(event EventTick
  (params (DeltaSeconds :type Float%20%28single-precision%29))
  (Transformation|SetWorldLocation (Variables|Default|GetNum) (+ (Transformation|GetActorLocation) "0.000000,0.000000,10.000000") false true))

(event EventExecute
  (CallFunction|HighLighting))

(event EventDemonstrate
  (CallFunction|PlayAnim))

(event EventReset
  (CallFunction|StopAnim)
  (Class|ActorSequenceComponent|PlaySequence (Variables|Default|GetStart%20State))
  (Variables|Default|SetToggle false)
  (CallFunction|SetText))

(fn ConstructionScript
  (|CallParentFunction))

(fn StopAnim
  (Class|ActorSequenceComponent|StopSequence (Variables|Default|GetHalf%20Tight))
  (Class|ActorSequenceComponent|StopSequence (Variables|Default|GetHalf%20to%20Full%20Tight))
  (Class|ActorSequenceComponent|StopSequence (Variables|Default|GetFull%20Tight))
  (Class|MovieSceneSequencePlayer|GotoEndandStop (Variables|/Script/ActorSequence.ActorSequenceComponent|GetSequencePlayer (Variables|Default|GetHighlight))))

(fn StopHighLight
  (Class|MovieSceneSequencePlayer|PlayLooping (Variables|/Script/ActorSequence.ActorSequenceComponent|GetSequencePlayer (Variables|Default|GetHighlight)) 0))

(fn HighLighting
  (Class|MovieSceneSequencePlayer|PlayLooping (Variables|/Script/ActorSequence.ActorSequenceComponent|GetSequencePlayer (Variables|Default|GetHighlight)) -1))

(fn PlayAnim
  (Class|MovieSceneSequencePlayer|PlayLooping (Variables|/Script/ActorSequence.ActorSequenceComponent|GetSequencePlayer (Variables|Default|GetHighlight)) 0))

(fn SetText
  (params (Text :type Text))
  (Default|SetNumText (Variables|Default|GetNumber%20Text) Text))