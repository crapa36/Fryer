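; BP_LEVEL9 is a level 9 actor that populates a leg with bolts when play begins.
; It enables player input, caches the BP_LV9_Leg from its Leg child actor, then adds a BP_LV9_Bolt1 child actor for every socket on the leg mesh.
; Each bolt takes its socket's transform, gets a slight local Z lift and is stored in Bolts.
; A loop playing bolt highlight sequences exists but is unconnected.
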(event EventBeginPlay
  (Input|EnableInput (Game|GetPlayerController 0))
  (bind _asbp_lv9_leg (Utilities|Casting|CastToBP_LV9_Leg (Variables|/Script/Engine.ChildActorComponent|GetChildActor (Variables|Default|GetLeg))))
  (Variables|Default|SetLeg%20Actor _asbp_lv9_leg)
  (CallFunction|SpawnBolt))

(event Collision|EventActorBeginOverlap
  (params (OtherActor :type Actor%20Object%20Reference)))

(event EventTick
  (params (DeltaSeconds :type Float%20%28single-precision%29)))

(fn ConstructionScript)

(fn SpawnBolt
  (bind _leg_actor (Variables|Default|GetLeg%20Actor))
  (bind _leg (Variables|/Game/UtesPelare/BP/LEVEL9/Components/BP_LV9_Leg.BP_LV9_Leg_C|GetLeg _leg_actor))
  (for _array_element (Transformation|GetAllSocketNames _leg)
    (bind _returnvalue (AddComponent|AddChildActorComponent false (Transformation|GetSocketTransform _leg _array_element "RTS_Actor")))
    (ChildActorComponent|SetChildActorClass _returnvalue "/Game/UtesPelare/BP/LEVEL9/Components/BP_LV9_Bolt1.BP_LV9_Bolt1_C")
    (Transformation|AddActorLocalOffset (Variables|/Script/Engine.ChildActorComponent|GetChildActor _returnvalue) "0.000000,0.000000,2.000000" false true)
    (bind _asbp_lv9_bolt_1 (Utilities|Casting|CastToBP_LV9_Bolt1 (Variables|/Script/Engine.ChildActorComponent|GetChildActor _returnvalue)))
    (Utilities|Array|Add (Variables|Default|GetBolts) _asbp_lv9_bolt_1)))