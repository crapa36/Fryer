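; Level 9 bolt component that animates a bolt being tightened and signals when it is done.
; Highlight loops while highlighting; PlayAnim or StopHighLight lets it finish, which chains into the FullTight sequence and then calls OnCompleted.
; SetOrign and SetComplete stop animations, hide the circle arrow, then restore the start state or jump to the fully tightened end frame.
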(event Custom|OnFinished_Event
  (Class|ActorSequenceComponent|PlaySequence (Variables|Default|GetFull%20Tight)))

(event Custom|Event%20Set%20Orign
  (CallFunction|StopAnim)
  (Class|ActorSequenceComponent|PlaySequence (Variables|Default|GetStart%20State)))

(event Custom|CustomEvent
  (Default|CallOnCompleted))

(event Custom|Event%20Set%20Complete
  (bind _full_tight (Variables|Default|GetFull%20Tight))
  (bind _sequenceplayer (Variables|/Script/ActorSequence.ActorSequenceComponent|GetSequencePlayer _full_tight))
  (CallFunction|StopAnim)
  (Sequencer|Player|Play _sequenceplayer :!class /Script/MovieScene.MovieSceneSequencePlayer)
  (Class|MovieSceneSequencePlayer|GotoEndandStop _sequenceplayer))

(event EventBeginPlay
  (EventDispatchers|AssignOnFinished (Variables|/Script/ActorSequence.ActorSequenceComponent|GetSequencePlayer (Variables|Default|GetFull%20Tight)) (delegate Custom|CustomEvent))
  (EventDispatchers|AssignOnFinished (Variables|/Script/ActorSequence.ActorSequenceComponent|GetSequencePlayer (Variables|Default|GetHighlight)) (delegate Custom|OnFinished_Event)))

(fn ConstructionScript
  (|CallParentFunction))

(fn StopAnim
  (Class|ActorSequenceComponent|StopSequence (Variables|Default|GetFull%20Tight))
  (Class|MovieSceneSequencePlayer|GotoEndandStop (Variables|/Script/ActorSequence.ActorSequenceComponent|GetSequencePlayer (Variables|Default|GetHighlight)))
  (Class|ActorSequenceComponent|PlaySequence (Variables|Default|GetHide%20CircleArrow)))

(fn StopHighLight
  (Class|MovieSceneSequencePlayer|PlayLooping (Variables|/Script/ActorSequence.ActorSequenceComponent|GetSequencePlayer (Variables|Default|GetHighlight)) 0))

(fn HighLighting
  (Class|MovieSceneSequencePlayer|PlayLooping (Variables|/Script/ActorSequence.ActorSequenceComponent|GetSequencePlayer (Variables|Default|GetHighlight)) -1))

(fn PlayAnim
  (Class|MovieSceneSequencePlayer|PlayLooping (Variables|/Script/ActorSequence.ActorSequenceComponent|GetSequencePlayer (Variables|Default|GetHighlight)) 0))