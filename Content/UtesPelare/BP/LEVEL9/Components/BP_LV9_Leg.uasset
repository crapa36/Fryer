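; BP_LV9_Leg is a level 9 leg component that manages a set of BP_LV9_Bolt actors and their highlights.
; SpawnBolts creates a bolt child actor at each Leg mesh socket, nudges it up and stores it in Bolts, but its graph call is unconnected.
; Pressing key 1 plays every stored bolt's Highlight sequence, though the EnableInput call is also unconnected.
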(event EventBeginPlay)

(event Input|KeyboardEvents|1
  (params (Key :type Key%20Structure))
  (:Pressed
    (for _array_element (Variables|Default|GetBolts)
      (Class|ActorSequenceComponent|PlaySequence (Variables|/Game/UtesPelare/BP/LEVEL9/Components/BP_LV9_Bolt.BP_LV9_Bolt_C|GetHighlight _array_element)))))

(fn ConstructionScript
  (|CallParentFunction))

(fn SpawnBolts
  (for (_array_element _array_index) (Transformation|GetAllSocketNames (Variables|Default|GetLeg))
    (bind _returnvalue (AddComponent|AddChildActorComponent false (Transformation|GetSocketTransform (Variables|Default|GetLeg) _array_element "RTS_World")))
    (ChildActorComponent|SetChildActorClass _returnvalue "/Game/UtesPelare/BP/LEVEL9/Components/BP_LV9_Bolt.BP_LV9_Bolt_C")
    (Transformation|AddActorLocalOffset (Variables|/Script/Engine.ChildActorComponent|GetChildActor _returnvalue) "0.000000,0.000000,2.000000" false true)
    (bind _asbp_lv9_bolt (Utilities|Casting|CastToBP_LV9_Bolt (Variables|/Script/Engine.ChildActorComponent|GetChildActor _returnvalue)))
    (Utilities|Array|Add (Variables|Default|GetBolts) _asbp_lv9_bolt)))