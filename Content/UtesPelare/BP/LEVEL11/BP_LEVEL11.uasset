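; BP_LEVEL11 is the level 11 actor in what appears to be a furniture assembly manual, presenting a table step.
; On BeginPlay it becomes the player's view target, enables input and has ManualInstance bind button clicks to sub-steps through the Blackboard's SubLevel key.
; It also rolls the TableTop half a turn when the game instance's DefaultShape flag is false.
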(event EventBeginPlay
  (bind _returnvalue (Game|GetPlayerController 0))
  (bind _returnvalue_2 (Game|GetGameInstance))
  (bind _asmanual_instance (Utilities|Casting|CastToManualInstance _returnvalue_2))
  (Game|Player|SetViewTargetwithBlend _returnvalue self 0.0 "VTBlend_Linear" 0.0 false)
  (Input|EnableInput _returnvalue)
  (Default|SetButtononClickedforSubStep _asmanual_instance (AI|GetBlackboard 0) "SubLevel" 2)
  (if (not (Variables|/Game/UtesPelare/BluePrints/sh/ManualInstance.ManualInstance_C|GetDefault%20Shape? _asmanual_instance))
    (Transformation|SetRelativeRotation (Variables|Default|GetTableTop) "0.000000,180.000000,0.000000" false false)))

(event Collision|EventActorBeginOverlap
  (params (OtherActor :type Actor%20Object%20Reference)))

(event EventTick
  (params (DeltaSeconds :type Float%20%28single-precision%29)))

(event Input|KeyboardEvents|RightBracket
  (params (Key :type Key%20Structure :default "None")))

(fn ConstructionScript)