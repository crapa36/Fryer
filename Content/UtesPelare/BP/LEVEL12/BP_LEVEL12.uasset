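; BP_LEVEL12 is the setup actor for level 12, which takes over the first player's view on BeginPlay.
; It has the ManualInstance game instance set up sub-step button clicks against its Blackboard's SubLevel key, capped at 2.
; When the game instance's DefaultShape flag is false, it rotates the TableTop component half a turn.
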(event EventBeginPlay
  (bind _returnvalue (Game|GetGameInstance))
  (bind _asmanual_instance (Utilities|Casting|CastToManualInstance _returnvalue))
  (Game|Player|SetViewTargetwithBlend (Game|GetPlayerController 0) self 0.0 "VTBlend_Linear" 0.0 false)
  (Default|SetButtononClickedforSubStep _asmanual_instance (AI|GetBlackboard 0) "SubLevel" 2)
  (if (not (Variables|/Game/UtesPelare/BluePrints/sh/ManualInstance.ManualInstance_C|GetDefault%20Shape? _asmanual_instance))
    (Transformation|SetRelativeRotation (Variables|Default|GetTableTop) "0.000000,180.000000,0.000000" false false)))

(event Collision|EventActorBeginOverlap
  (params (OtherActor :type Actor%20Object%20Reference)))

(event EventTick
  (params (DeltaSeconds :type Float%20%28single-precision%29)))

(fn ConstructionScript)