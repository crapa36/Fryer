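; BP_Level2_Pawn is the Level 2 pawn that coordinates animated BP_Level2_Body child actors and serves as the player's view target.
; On BeginPlay it registers itself as each body's Manager and hooks ManualInstance's sub-step buttons to the "Sub Level" blackboard key.
; CallExecute triggers every body behind an Animating guard.
; CallFinished clears the guard after a short delay and signals assembly completion.
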(event EventBeginPlay
  (Game|Player|SetViewTargetwithBlend (Game|GetPlayerController 0) self 0.0 "VTBlend_Linear" 0.0 false)
  (for _array_element (Actor|GetAllChildActors true)
    (bind _asbp_level_2_body (Utilities|Casting|CastToBP_Level2_Body _array_element))
    (Utilities|Array|Add (Variables|Default|GetBodys) _asbp_level_2_body)
    (Variables|/Game/UtesPelare/BluePrints/LMS/Level2/BP_Level2_Body.BP_Level2_Body_C|SetManager _asbp_level_2_body self))
  (bind _asmanual_instance (Utilities|Casting|CastToManualInstance (Game|GetGameInstance)))
  (Default|SetButtononClickedforSubStep _asmanual_instance (AI|GetBlackboard 0) "Sub Level" 2))

(event Collision|EventActorBeginOverlap
  (params (OtherActor :type Actor%20Object%20Reference)))

(event EventCallExecute
  (if (not (Variables|Default|GetAnimating))
    (Variables|Default|SetAnimating true)
    (for _array_element (Variables|Default|GetBodys)
      (Class|BPIAssemblyManager|CallExecute(Message) _array_element))))

(event EventCallFinished
  (Utilities|FlowControl|Delay 0.2)
  (Variables|Default|SetAnimating false)
  (Default|CallOnAssemblyComplete))

(event EventTick
  (params (DeltaSeconds :type Float%20%28single-precision%29)))

(fn ConstructionScript)