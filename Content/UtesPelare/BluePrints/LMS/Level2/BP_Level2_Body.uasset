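; Level 2 body actor in the LMS content, with a click-adjustable height and a leg-insertion animation that reports completion to its Manager.
; Seven clickable box colliders each pick a height step, and ChangeHeight plays only the span between current and target using mirrored forward and backward Actor Sequences, treating height as sequence time.
; CallExecute plays LegInsert, whose finish calls the Manager's finished message, while CallReset is empty.
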(event OnClicked(BoxCollider6)
  (params (TouchedComponent :type Primitive%20Component%20Object%20Reference) (ButtonPressed :type Key%20Structure))
  (CallFunction|ChangeHeight 6.0))

(event OnClicked(BoxCollider4)
  (params (TouchedComponent :type Primitive%20Component%20Object%20Reference) (ButtonPressed :type Key%20Structure))
  (CallFunction|ChangeHeight 4.0))

(event OnClicked(BoxCollider3)
  (params (TouchedComponent :type Primitive%20Component%20Object%20Reference) (ButtonPressed :type Key%20Structure))
  (CallFunction|ChangeHeight 3.0))

(event OnClicked(BoxCollider1)
  (params (TouchedComponent :type Primitive%20Component%20Object%20Reference) (ButtonPressed :type Key%20Structure))
  (CallFunction|ChangeHeight 1.0))

(event OnClicked(BoxCollider2)
  (params (TouchedComponent :type Primitive%20Component%20Object%20Reference) (ButtonPressed :type Key%20Structure))
  (CallFunction|ChangeHeight 2.0))

(event OnClicked(BoxCollider0)
  (params (TouchedComponent :type Primitive%20Component%20Object%20Reference) (ButtonPressed :type Key%20Structure))
  (CallFunction|ChangeHeight 0.0))

(event OnClicked(BoxCollider5)
  (params (TouchedComponent :type Primitive%20Component%20Object%20Reference) (ButtonPressed :type Key%20Structure))
  (CallFunction|ChangeHeight 5.0))

(event Custom|On%20Complete
  (Class|BPIAssemblyManager|CallFinished(Message) (Variables|Default|GetManager)))

(event EventBeginPlay
  (bind _leginsert (Variables|Default|GetLegInsert))
  (bind _sequenceplayer (Variables|/Script/ActorSequence.ActorSequenceComponent|GetSequencePlayer _leginsert))
  (Components|Timeline|SetPlaybackPosition _sequenceplayer (Utilities|Struct|MakeMovieSceneSequencePlaybackParams "(FrameNumber=(Value=0),SubFrame=0.000000)" 0.0 "" "(Hours=0,Minutes=0,Seconds=0,Frames=0,Subframe=0.000000,bDropFrameFormat=False)" "Frame" "Play" true))
  (EventDispatchers|AssignOnFinished _sequenceplayer (delegate Custom|On%20Complete)))

(event Collision|EventActorBeginOverlap
  (params (OtherActor :type Actor%20Object%20Reference)))

(event EventTick
  (params (DeltaSeconds :type Float%20%28single-precision%29)))

(event EventCallReset)

(event EventCallExecute
  (Class|ActorSequenceComponent|PlaySequence (Variables|Default|GetLegInsert)))

(fn ConstructionScript)

(fn ChangeHeight
  (params (Target%20Height :type Float%20%28double-precision%29))
  (bind _actorsequence_forward (Variables|Default|GetActorSequence_Forward))
  (bind _actorsequence_backward (Variables|Default|GetActorSequence_Backward))
  (bind _sequenceplayer (Variables|/Script/ActorSequence.ActorSequenceComponent|GetSequencePlayer _actorsequence_forward))
  (bind _sequenceplayer_2 (Variables|/Script/ActorSequence.ActorSequenceComponent|GetSequencePlayer _actorsequence_backward))
  (LocalVariables|SetTempNowHeight (Variables|Default|GetNowHeight))
  (Variables|Default|SetNowHeight Target%20Height)
  (Class|ActorSequenceComponent|StopSequence (Variables|Default|GetActorSequence_Backward))
  (if (< (LocalVariables|GetTempNowHeight) Target%20Height)
    (Class|MovieSceneSequencePlayer|SetTimeRange _sequenceplayer (LocalVariables|GetTempNowHeight) (- Target%20Height (LocalVariables|GetTempNowHeight)))
    (Sequencer|Player|Play _sequenceplayer :!class /Script/MovieScene.MovieSceneSequencePlayer)
    (else
      (Class|MovieSceneSequencePlayer|SetTimeRange _sequenceplayer_2 (- 6.0 (LocalVariables|GetTempNowHeight)) (- (LocalVariables|GetTempNowHeight) Target%20Height))
      (Sequencer|Player|Play _sequenceplayer_2 :!class /Script/MovieScene.MovieSceneSequencePlayer))))