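; BP_Level1_Pawn is the Level 1 pawn that serves as view target and manager for an assembly animation of its child BP_Level1_Body actors.
; On BeginPlay it collects the bodies, sets itself as their Manager and configures ManualInstance's sub-step button against the "Sub Level" blackboard key.
; CallExecute messages every body except the first, guarded by an Animating flag.
; CallFinished clears the flag after a short delay and signals assembly completion.
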(event EventBeginPlay
  (Game|Player|SetViewTargetwithBlend (Game|GetPlayerController 0) self 0.0 "VTBlend_Linear" 0.0 false)
  (for _array_element (Actor|GetAllChildActors true)
    (bind _asbp_level_1_body (Utilities|Casting|CastToBP_Level1_Body _array_element))
    (Utilities|Array|Add (Variables|Default|GetBodys) _asbp_level_1_body)
    (Variables|/Game/UtesPelare/BluePrints/LMS/Level1/BP_Level1_Body.BP_Level1_Body_C|SetManager _asbp_level_1_body self))
  (bind _asmanual_instance (Utilities|Casting|CastToManualInstance (Game|GetGameInstance)))
  (Default|SetButtononClickedforSubStep _asmanual_instance (AI|GetBlackboard 0) "Sub Level" 1))

(event Collision|EventActorBeginOverlap
  (params (OtherActor :type Actor%20Object%20Reference)))

(event EventTick
  (params (DeltaSeconds :type Float%20%28single-precision%29)))

(event EventCallExecute
  (if (not (Variables|Default|GetAnimating))
    (Variables|Default|SetAnimating true)
    (for (_array_element _array_index) (Variables|Default|GetBodys)
      (if (!= _array_index 0)
        (Class|BPIAssemblyManager|CallExecute(Message) _array_element)))))

(event EventCallFinished
  (Utilities|FlowControl|Delay 0.2)
  (Variables|Default|SetAnimating false)
  (Default|CallOnAssemblyComplete))

(fn ConstructionScript)