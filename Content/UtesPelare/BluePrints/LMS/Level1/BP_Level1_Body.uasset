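; Level 1 body actor that plays its actor sequence as a step reporting to a Manager.
; BeginPlay resets the playback position and binds the finish callback, CallExecute plays the sequence, and completion calls CallFinishedMessage on the Manager.
; An Execute macro, not invoked in these graphs, blinks an arrow twice with delays, then reveals the hand UI.
; CallReset is empty.
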(event Custom|On%20Complete
  (Class|BPIAssemblyManager|CallFinished(Message) (Variables|Default|GetManager)))

(event EventBeginPlay
  (bind _actorsequence (Variables|Default|GetActorSequence))
  (bind _sequenceplayer (Variables|/Script/ActorSequence.ActorSequenceComponent|GetSequencePlayer _actorsequence))
  (Components|Timeline|SetPlaybackPosition _sequenceplayer (Utilities|Struct|MakeMovieSceneSequencePlaybackParams "(FrameNumber=(Value=0),SubFrame=0.000000)" 0.0 "" "(Hours=0,Minutes=0,Seconds=0,Frames=0,Subframe=0.000000,bDropFrameFormat=False)" "Frame" "Play" true))
  (EventDispatchers|AssignOnFinished _sequenceplayer (delegate Custom|On%20Complete)))

(event Collision|EventActorBeginOverlap
  (params (OtherActor :type Actor%20Object%20Reference)))

(event EventTick
  (params (DeltaSeconds :type Float%20%28single-precision%29)))

(event EventCallReset)

(event EventCallExecute
  (Class|ActorSequenceComponent|PlaySequence (Variables|Default|GetActorSequence)))

(fn ConstructionScript)