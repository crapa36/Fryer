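; Body actor for Level 4 in the LMS content, holding bolt child actors and reporting to a Manager when their sequences finish.
; On BeginPlay it collects the bolts into an array, sets each one's ActorSequence playback position and binds its OnFinished event.
; Each finished sequence calls the Manager's finished message separately.
; Execute and Reset events are empty, and a PlaySequence call is left unconnected.
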(event Custom|On%20Complete
  (Class|BPIAssemblyManager|CallFinished(Message) (Variables|Default|GetManager)))

(event EventBeginPlay
  (for _array_element (Actor|GetAllChildActors true)
    (bind _asbp_level_4_bolt (Utilities|Casting|CastToBP_Level4_Bolt _array_element))
    (Utilities|Array|Add (Variables|Default|GetBolts) _asbp_level_4_bolt)
    (Components|Timeline|SetPlaybackPosition (Variables|/Script/ActorSequence.ActorSequenceComponent|GetSequencePlayer (Variables|/Game/UtesPelare/BluePrints/LMS/Level4/BP_Level4_Bolt.BP_Level4_Bolt_C|GetActorSequence _asbp_level_4_bolt)) (Utilities|Struct|MakeMovieSceneSequencePlaybackParams "(FrameNumber=(Value=0),SubFrame=0.000000)" 0.0 "" "(Hours=0,Minutes=0,Seconds=0,Frames=0,Subframe=0.000000,bDropFrameFormat=False)" "Frame" "Play" true))
    (EventDispatchers|AssignOnFinished (Variables|/Script/ActorSequence.ActorSequenceComponent|GetSequencePlayer (Variables|/Game/UtesPelare/BluePrints/LMS/Level4/BP_Level4_Bolt.BP_Level4_Bolt_C|GetActorSequence _asbp_level_4_bolt)) (delegate Custom|On%20Complete))))

(event Collision|EventActorBeginOverlap
  (params (OtherActor :type Actor%20Object%20Reference)))

(event EventTick
  (params (DeltaSeconds :type Float%20%28single-precision%29)))

(event EventCallReset)

(event EventCallExecute)

(fn ConstructionScript)