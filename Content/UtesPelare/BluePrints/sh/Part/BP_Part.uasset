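; BP_Part is a clickable part actor with a name label that registers itself with the PartPC player controller when clicked.
; On BeginPlay it caches that controller and writes its Text into the PartName widget.
; Helper functions yaw and pitch RotationCenter in world space, return its local bounds midpoint, and hide the actor or label.
; DisableObject hides the actor and turns off collision, but sets tick enabled despite its comment.
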(event EventBeginPlay
  (bind _aspart_pc (Utilities|Casting|CastToPartPC (Game|GetPlayerController 0)))
  (Variables|Default|SetPart%20PC _aspart_pc)
  (bind _aspart_text_wbp (Utilities|Casting|CastToPartTextWBP (UserInterface|GetWidget (Variables|Default|GetPart%20Name))))
  (Default|SetText _aspart_text_wbp (Variables|Default|GetText)))

(event Collision|EventActorBeginOverlap
  (params (OtherActor :type Actor%20Object%20Reference)))

(event EventTick
  (params (DeltaSeconds :type Float%20%28single-precision%29)))

(event MouseInput|EventActorOnClicked
  (params (ButtonPressed :type Key%20Structure :default "None"))
  (bind _part_pc (Variables|Default|GetPart%20PC))
  (Utilities|IsValid _part_pc
    (:Is%20Valid
      (Default|SetObject _part_pc self))))

(fn ConstructionScript)

(fn HideObject
  (Rendering|SetActorHiddenInGame true))

(fn HideText
  (Development|SetHiddeninGame (Variables|Default|GetPart%20Name) true true))

(fn GetSMMidPoint
  (bind _rotation_center (Variables|Default|GetRotation%20Center))
  (bind (_min _max) (Components|StaticMesh|GetLocalBounds _rotation_center))
  (return (/ (+ _min _max) 2.0)))

(fn RotationSM
  (params (dx :type Float%20%28double-precision%29) (dy :type Float%20%28double-precision%29))
  (bind _rotation_center (Variables|Default|GetRotation%20Center))
  (Transformation|AddWorldRotation _rotation_center (Math|Rotator|MakeRotator 0.0 0.0 dx) false false)
  (Transformation|AddWorldRotation _rotation_center (Math|Rotator|MakeRotator 0.0 dy 0.0) false false))

(fn DisableObject
  ;[0.15 0.15 0.15 0.5] 안보이고, 충돌 무시하고, Tick Event 안받게 == Unity Enable (False)
  (CallFunction|HideObject)
  (Collision|SetActorEnableCollision false)
  (Actor|Tick|SetActorTickEnabled true))