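; ProhibitionActor is an actor that plays a blinking level sequence, judging by its name as a prohibition indicator.
; Demonstrate and Execute both play the Blinking sequence with a loop count of zero.
; When that sequence finishes, a handler bound at BeginPlay fires the OnCompeleted dispatcher.
; Reset clears all listeners from that dispatcher and plays the StartState sequence.
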(event Custom|OnFinished
  (Default|CallOnCompeleted))

(event EventBeginPlay
  (EventDispatchers|BindEventtoOnFinished (Variables|/Script/ActorSequence.ActorSequenceComponent|GetSequencePlayer (Variables|Default|GetBlinking)) (delegate Custom|OnFinished)))

(event EventReset
  (EventDispatchers|UnbindallEventsfromOnCompeleted)
  (Class|ActorSequenceComponent|PlaySequence (Variables|Default|GetStart%20State)))

(event EventDemonstrate
  (Class|MovieSceneSequencePlayer|PlayLooping (Variables|/Script/ActorSequence.ActorSequenceComponent|GetSequencePlayer (Variables|Default|GetBlinking)) 0))

(event EventExecute
  (Class|MovieSceneSequencePlayer|PlayLooping (Variables|/Script/ActorSequence.ActorSequenceComponent|GetSequencePlayer (Variables|Default|GetBlinking)) 0))

(fn ConstructionScript)