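; Manager for a step-by-step manual, driving the ExplainUI widget and level switching between part view and explanation mode.
; It tracks the step index, updating step text and Prev/Next clickability; step changes open PartMap, while Explain opens the matching numbered Level map.
; For sub-steps, it rebinds Prev/Next to adjust a Blackboard integer, restoring whole-step navigation at either bound.
; Helpers open menu and caution maps or spawn a target actor.
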(event Custom|Set%20Prev%20Button%20For%20SubStep
  (params (BlackBoard :type Blackboard%20Component%20Object%20Reference) (Key%20Name :type Name))
  (bind _explain_ui (Variables|Widget|GetExplain%20UI))
  (bind _prevbutton (Variables|/Game/UtesPelare/Widget/ExplainWBP.ExplainWBP_C|GetPrevButton _explain_ui))
  (EventDispatchers|UnbindallEventsfromOnClicked _prevbutton)
  (EventDispatchers|AssignOnClicked _prevbutton (delegate Custom|Set%20Prev%20OnClicked)))

(event Custom|Set%20Next%20Button%20OnClicked
  (bind _explain_ui (Variables|Widget|GetExplain%20UI))
  (bind _nextbutton (Variables|/Game/UtesPelare/Widget/ExplainWBP.ExplainWBP_C|GetNextButton _explain_ui))
  (if (== (Class|BlackboardComponent|GetValueasInt (stale Custom|Set%20Next%20Button%20For%20SubStep BlackBoard) (stale Custom|Set%20Next%20Button%20For%20SubStep Key%20Name)) (stale Custom|Set%20Next%20Button%20For%20SubStep max))
    (EventDispatchers|UnbindallEventsfromOnClicked _nextbutton)
    (EventDispatchers|AssignOnClicked _nextbutton (delegate Custom|Restore%20Next%20Button%20OnClicked))
    (CallFunction|PressedNextButton)
    (else
      (Class|BlackboardComponent|SetValueasInt (stale Custom|Set%20Next%20Button%20For%20SubStep BlackBoard) (stale Custom|Set%20Next%20Button%20For%20SubStep Key%20Name) (+ (Class|BlackboardComponent|GetValueasInt (stale Custom|Set%20Next%20Button%20For%20SubStep BlackBoard) (stale Custom|Set%20Next%20Button%20For%20SubStep Key%20Name)) 1))
      (CallFunction|SetSubStepText (Class|BlackboardComponent|GetValueasInt (stale Custom|Set%20Next%20Button%20For%20SubStep BlackBoard) (stale Custom|Set%20Next%20Button%20For%20SubStep Key%20Name)))
      (CallFunction|ValidateButtonJudgment true (Class|BlackboardComponent|GetValueasInt (stale Custom|Set%20Next%20Button%20For%20SubStep BlackBoard) (stale Custom|Set%20Next%20Button%20For%20SubStep Key%20Name)) (stale Custom|Set%20Next%20Button%20For%20SubStep max)))))

(event Custom|Restore%20Prev%20OnClicked
  (CallFunction|PressedPrevButton))

(event Custom|Restore%20Next%20Button
  (CallFunction|PressedNextButton))

(event Custom|Init%20MI
  (bind _explain_ui (Variables|Widget|GetExplain%20UI))
  (bind _nextbutton (Variables|/Game/UtesPelare/Widget/ExplainWBP.ExplainWBP_C|GetNextButton _explain_ui))
  (bind _prevbutton (Variables|/Game/UtesPelare/Widget/ExplainWBP.ExplainWBP_C|GetPrevButton _explain_ui))
  (Utilities|IsValid _explain_ui
    (:Is%20Valid
      (Variables|Default|Setidx 1)
      (Variables|Default|SetExplain%20Mode? false)
      (EventDispatchers|UnbindallEventsfromOnClicked _nextbutton)
      (EventDispatchers|AssignOnClicked _nextbutton (delegate Custom|Restore%20Next%20Button))
      (CallFunction|PressedNextButton)
      (EventDispatchers|UnbindallEventsfromOnClicked _prevbutton)
      (EventDispatchers|AssignOnClicked _prevbutton (delegate Custom|Restore%20Prev%20Button))
      (CallFunction|PressedPrevButton))))

(event Custom|Set%20Prev%20OnClicked
  (bind _explain_ui (Variables|Widget|GetExplain%20UI))
  (bind _prevbutton (Variables|/Game/UtesPelare/Widget/ExplainWBP.ExplainWBP_C|GetPrevButton _explain_ui))
  (if (== (Class|BlackboardComponent|GetValueasInt (stale Custom|Set%20Prev%20Button%20For%20SubStep BlackBoard) (stale Custom|Set%20Prev%20Button%20For%20SubStep Key%20Name)) 0)
    (EventDispatchers|UnbindallEventsfromOnClicked _prevbutton)
    (EventDispatchers|AssignOnClicked _prevbutton (delegate Custom|Restore%20Prev%20OnClicked))
    (CallFunction|PressedPrevButton)
    (else
      (Class|BlackboardComponent|SetValueasInt (stale Custom|Set%20Prev%20Button%20For%20SubStep BlackBoard) (stale Custom|Set%20Prev%20Button%20For%20SubStep Key%20Name) (- (Class|BlackboardComponent|GetValueasInt (stale Custom|Set%20Prev%20Button%20For%20SubStep BlackBoard) (stale Custom|Set%20Prev%20Button%20For%20SubStep Key%20Name)) 1))
      (CallFunction|SetSubStepText (Class|BlackboardComponent|GetValueasInt (stale Custom|Set%20Prev%20Button%20For%20SubStep BlackBoard) (stale Custom|Set%20Prev%20Button%20For%20SubStep Key%20Name)))
      (CallFunction|ValidateButtonJudgment true (Class|BlackboardComponent|GetValueasInt (stale Custom|Set%20Prev%20Button%20For%20SubStep BlackBoard) (stale Custom|Set%20Prev%20Button%20For%20SubStep Key%20Name))))))

(event Custom|Restore%20Prev%20Button
  (CallFunction|PressedPrevButton))

(event Custom|Set%20Button%20OnClicked%20For%20SubStep
  (params (BlackBoard :type Blackboard%20Component%20Object%20Reference) (Key%20Name :type Name) (Max :type Integer))
  (CallFunction|SetSubStepText (Class|BlackboardComponent|GetValueasInt BlackBoard Key%20Name))
  (CallFunction|SetPrevButtonforSubStep BlackBoard Key%20Name)
  (CallFunction|SetNextButtonforSubStep BlackBoard Key%20Name Max))

(event Custom|Set%20Next%20Button%20For%20SubStep
  (params (BlackBoard :type Blackboard%20Component%20Object%20Reference) (Key%20Name :type Name) (max :type Integer))
  (bind _explain_ui (Variables|Widget|GetExplain%20UI))
  (bind _nextbutton (Variables|/Game/UtesPelare/Widget/ExplainWBP.ExplainWBP_C|GetNextButton _explain_ui))
  (EventDispatchers|UnbindallEventsfromOnClicked _nextbutton)
  (EventDispatchers|AssignOnClicked _nextbutton (delegate Custom|Set%20Next%20Button%20OnClicked)))

(event Custom|Restore%20Next%20Button%20OnClicked
  (CallFunction|PressedNextButton))

(fn ShowUI
  (bind _returnvalue (Game|GetPlayerController 0))
  (Utilities|IsValid (Variables|Widget|GetExplain%20UI)
    (:Is%20Valid
      _)
    (:Is%20Not%20Valid
      (bind _returnvalue_2 (UserInterface|CreateWidget "/Game/UtesPelare/Widget/ExplainWBP.ExplainWBP_C" _returnvalue))
      (Variables|Widget|SetExplain%20UI _returnvalue_2)))
  (UserInterface|Viewport|AddtoViewport (Variables|Widget|GetExplain%20UI) 10)
  (Widget|SetVisibility (Variables|Widget|GetExplain%20UI) "SelfHitTestInvisible")
  (Variables|/Script/Engine.PlayerController|SetbShowMouseCursor _returnvalue true)
  (CallFunction|ValidateButtonJudgment false))

(fn PressedExplainButton
  (if (Variables|Default|GetFocus%20Part?)
    (Game|OpenLevel(byName) "PartMap")
    (Variables|Default|SetFocus%20Part? false)
    (else
      (bind _output_get (Variables|Default|SetExplain%20Mode? true))
      (Default|SetWidgetMode (Variables|Widget|GetExplain%20UI) _output_get)
      (CallFunction|ShowNowStepExplain))))

(fn PressedPrevButton
  (bind _explain_ui (Variables|Widget|GetExplain%20UI))
  (if (> (Variables|Default|Getidx) 1)
    (bind _result (Math|Integer|DecrementInt (Variables|Default|Getidx))
      (:%20%20
        (bind _output_get (Variables|Default|Setidx _result))
        (Default|SetStepText _explain_ui (Utilities|Array|Get(acopy) (Variables|Default|GetStep%20To%20Text) _output_get))
        (CallFunction|ValidateButtonJudgment false)
        (CallFunction|SetPartMode)
        (Default|SetText _explain_ui)))))

(fn PressedNextButton
  (bind _explain_ui (Variables|Widget|GetExplain%20UI))
  (if (< (Variables|Default|Getidx) (Variables|Default|GetMax%20Step))
    (bind _result (Math|Integer|IncrementInt (Variables|Default|Getidx))
      (:%20%20
        (bind _output_get (Variables|Default|Setidx _result))
        (Default|SetStepText _explain_ui (Utilities|Array|Get(acopy) (Variables|Default|GetStep%20To%20Text) _output_get))
        (CallFunction|ValidateButtonJudgment false)
        (CallFunction|SetPartMode)
        (Default|SetText _explain_ui)))))

(fn SetPartMode
  (bind _output_get (Variables|Default|SetExplain%20Mode? false))
  (Default|SetWidgetMode (Variables|Widget|GetExplain%20UI) _output_get)
  (CallFunction|ShowNowStepPart))

(fn ShowNowStepPart
  (Game|OpenLevel(byName) (Utilities|Name|MakeLiteralName "PartMap")))

(fn ShowNowStepExplain
  (Game|OpenLevel(byName) (Utilities|Name|MakeLiteralName (Utilities|String|StringToName (Utilities|String|BuildString(Name) "" "" (Utilities|Name|MakeLiteralName "Level") (Utilities|String|ToString(Integer) (Variables|Default|Getidx)))))))

(fn ValidateButtonJudgment
  (params (Is%20SubStep? :type Boolean) (Now%20SubStep :type Integer) (Max%20SubStep :type Integer))
  (bind _explain_ui (Variables|Widget|GetExplain%20UI))
  (bind _explain_ui_2 (Variables|Widget|GetExplain%20UI))
  (LocalVariables|SetLowest 1)
  (LocalVariables|SetHighest (Variables|Default|GetMax%20Step))
  (if Is%20SubStep?
    (Default|SetPrevButtonClickable _explain_ui_2 (or (> (Variables|Default|Getidx) (LocalVariables|GetLowest)) (> Now%20SubStep 0)))
    (Default|SetNextButtonClickable _explain_ui_2 (or (< (Variables|Default|Getidx) (LocalVariables|GetHighest)) (< Now%20SubStep Max%20SubStep)))
    (else
      (Default|SetPrevButtonClickable _explain_ui (> (Variables|Default|Getidx) (LocalVariables|GetLowest)))
      (Default|SetNextButtonClickable _explain_ui (< (Variables|Default|Getidx) (LocalVariables|GetHighest))))))

(fn SetTextUI
  (params (str :type String))
  (Default|SetText (Variables|Widget|GetExplain%20UI) str))

(fn SetNowStep
  (params (step :type Integer) (substep? :type Boolean))
  (bind _explain_ui (Variables|Widget|GetExplain%20UI))
  (bind _output_get (Variables|Default|SetExplain%20Mode? true))
  (Default|SetWidgetMode (Variables|Widget|GetExplain%20UI) _output_get)
  (if (and (> step 0) (<= step (Variables|Default|GetMax%20Step)))
    (Variables|Default|Setidx step)
    (Utilities|IsValid _explain_ui
      (:Is%20Valid
        _)
      (:Is%20Not%20Valid
        (CallFunction|ShowUI)))
    (if substep?
      (CallFunction|SetSubStepText)
      (else
        (Default|SetStepText _explain_ui (Utilities|Text|ToText(Integer) (Variables|Default|Getidx)))))
    (CallFunction|ValidateButtonJudgment false)))

(fn SetSubStepText
  (params (Sub%20Step :type Integer))
  (Default|SetStepText (Variables|Widget|GetExplain%20UI) (Utilities|Text|ToText(String) (Utilities|String|BuildString(Integer) (Utilities|String|Append (Utilities|String|ToString(Integer) (Variables|Default|Getidx)) "-") "" Sub%20Step))))

(fn SpawnTargetActor
  (Game|SpawnActorfromClass (Variables|Default|GetTarget) (Math|Transform|MakeTransform "0, 0, 0") "AlwaysSpawn" "MultiplyWithRoot" 0 0))

(fn OpenMainMenuLevel
  (Game|OpenLevel(byName) "MainMenu"))

(fn OpenCautionLevel
  ;[0.15 0.15 0.15 0.5] TODO
  (Game|OpenLevel(byName) "CautionMap"))